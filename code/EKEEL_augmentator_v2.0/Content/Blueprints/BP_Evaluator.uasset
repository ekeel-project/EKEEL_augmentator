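; BP_Evaluator tracks how a user matches concepts by ID and scores the results.
; FirstMatch timestamps a concept, then Match counts attempts until a correct one records the solve time and duration.
; Each solve is sent to the Logger, followed by a ScoreSummary that is marked as testing-only.
; The summary logs a score from solved-to-attempt ratio, scaled down when average solve time exceeds a minute.
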(event EventBeginPlay
  (Variables|Default|GetLogger
    (:then)
    (:else
      (if (Variables|Default|GetLog)
        (Development|PrintString "[Warning][Evaluator] Logger not specified")))))

(fn ConstructionScript)

(fn Match
  (params (ConceptID :type String) (Correct :type Boolean))
  (bind _matchcount (Variables|Default|GetMatchCount))
  (bind (_value _returnvalue) (Utilities|Map|Find _matchcount ConceptID))
  (if (not (.ReturnValue (Utilities|Map|Find (Variables|Default|GetSolved) ConceptID))) ; Update only if unsolved
    (if (.ReturnValue (Utilities|Map|Find (Variables|Default|GetTimeFirstMatch) ConceptID))
      (if _returnvalue
        (Utilities|Map|Add (Variables|Default|GetMatchCount) ConceptID (+ _value 1))
        (else
          (Utilities|Map|Add (Variables|Default|GetMatchCount) ConceptID 1)))
      (if Correct ; Update solved only if correct
        (Utilities|Map|Add (Variables|Default|GetTimeToSolved) ConceptID (Math|DateTime|Now))
        (Utilities|Map|Add (Variables|Default|GetSolved) ConceptID (- (Math|Timespan|GetTotalSeconds (TimeOfDay|GetTimeOfDay (Math|DateTime|Now) :!class /Script/Engine.KismetMathLibrary)) (Math|Timespan|GetTotalSeconds (TimeOfDay|GetTimeOfDay (.Value (Utilities|Map|Find (Variables|Default|GetTimeFirstMatch) ConceptID)) :!class /Script/Engine.KismetMathLibrary))))
        (CallFunction|ConceptSolve ConceptID :!pinned true) ; Send evaluation
        ;[1 0.07677 0] FOR TESTING ONLY
        ; calls score summary every correct match
        ; (TODO): determine when app should fire this function
        (CallFunction|ScoreSummary)))))

(fn ConceptSolve
  (params (conceptID :type String))
  (bind _logger (Variables|Default|GetLogger)
    (:then
      (Default|LogAction _logger (Variables|Default|GetLog) "NewEnumerator19" conceptID (Utilities|String|ToString(Text) (Class|KismetTextLibrary|AsTimeDateTime (.Value (Utilities|Map|Find (Variables|Default|GetTimeFirstMatch) conceptID)))) (Utilities|String|ToString(Text) (Class|KismetTextLibrary|AsTimeDateTime (.Value (Utilities|Map|Find (Variables|Default|GetTimeToSolved) conceptID)))) (Utilities|String|ToString(Float) (.Value (Utilities|Map|Find (Variables|Default|GetSolved) conceptID))) (Utilities|String|ToString(Integer) (.Value (Utilities|Map|Find (Variables|Default|GetMatchCount) conceptID)))))
    (:else)))

(fn ScoreSummary
  (bind _returnvalue (Math|Float|MakeLiteralFloat 6e+01))
  (Utilities|FlowControl|Sequence
    (:then_0
      (bind _values (Utilities|Map|Values (Variables|Default|GetMatchCount)))
      (LocalVariables|SetTotalMatches 0)
      (for _array_element _values
        (LocalVariables|SetTotalMatches (+ (LocalVariables|GetTotalMatches) _array_element))))
    (:then_1
      (bind _values_2 (Utilities|Map|Values (Variables|Default|GetSolved)))
      (LocalVariables|SetAverageDuration 0.0)
      (for _array_element_2 _values_2
        (LocalVariables|SetAverageDuration (+ _array_element_2 (LocalVariables|GetAverageDuration))))
      (LocalVariables|SetAverageDuration (/ (LocalVariables|GetAverageDuration) (Utilities|Map|Length (Variables|Default|GetSolved)))))
    (:then_2
      (LocalVariables|SetScore (* (* (/ (Utilities|Map|Length (Variables|Default|GetSolved)) (LocalVariables|GetTotalMatches)) (Class|KismetSystemLibrary|MakeLiteralInteger 100)) (/ _returnvalue (Math|Float|Max(Float) _returnvalue (LocalVariables|GetAverageDuration))))))
    (:then_3
      (bind _logger (Variables|Default|GetLogger)
        (:then
          (Default|LogAction _logger (Variables|Default|GetLog) "NewEnumerator20" (Utilities|String|ToString(Integer) (Utilities|Map|Length (Variables|Default|GetSolved))) (Utilities|String|ToString(Integer) (LocalVariables|GetTotalMatches)) (Utilities|String|ToString(Float) (LocalVariables|GetAverageDuration)) (Utilities|String|ToString(Float) (LocalVariables|GetScore))))
        (:else)))))

(fn FirstMatch
  (params (concept_id :type String))
  (if (not (.ReturnValue (Utilities|Map|Find (Variables|Default|GetTimeFirstMatch) concept_id)))
    (Utilities|Map|Add (Variables|Default|GetTimeFirstMatch) concept_id (Math|DateTime|Now))))