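; BP_AnnotationMenu hosts an annotation menu widget for browsing annotations tied to concept data.
; The construction script creates a WBP_AnnotationMenu and assigns it to the AnnotationMenuWidget component.
; OpenMenu passes concept and annotation data to the widget to initialise its entries.
; SelectUp and SelectDown forward previous and next entry selection to the widget, retrieved through a cast helper.
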(fn ConstructionScript
  (bind _returnvalue (Game|ConstructObjectfromClass "/Game/Widgets/WBP_AnnotationMenu.WBP_AnnotationMenu_C"))
  (UserInterface|SetWidget (Variables|Default|GetAnnotationMenuWidget) _returnvalue))

(fn OpenMenu
  (params (ConceptData :type S%20Concept%20Structure) (AnnotationsData :type Array%20of%20S%20Concept%20Annotation%20Structures))
  (bind _annotationmenu (CallFunction|GetAnnotationMenuWidget))
  (Utilities|IsValid _annotationmenu
    (:Is%20Valid
      (Default|InitialiseEntries _annotationmenu ConceptData AnnotationsData :!pinned true) ; Send the concept and annotations to the widget\nfor initialisation
    )))

(fn GetAnnotationMenuWidget
  (bind _aswbp_annotation_menu (Utilities|Casting|CastToWBP_AnnotationMenu (UserInterface|GetWidget (Variables|Default|GetAnnotationMenuWidget))))
  (return _aswbp_annotation_menu) ; Retrieves the widget reference within the component
)

(fn SelectUp
  (bind _annotationmenu (CallFunction|GetAnnotationMenuWidget))
  (bind _aswbp_annotation_menu (Utilities|Casting|CastToWBP_AnnotationMenu _annotationmenu))
  (Default|SelectUp _aswbp_annotation_menu))

(fn SelectDown
  (bind _annotationmenu (CallFunction|GetAnnotationMenuWidget))
  (bind _aswbp_annotation_menu (Utilities|Casting|CastToWBP_AnnotationMenu _annotationmenu))
  (Default|SelectDown _aswbp_annotation_menu))