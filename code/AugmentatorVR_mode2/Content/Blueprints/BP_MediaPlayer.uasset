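; Media player actor that opens, pauses and resumes media by ID on a MediaPlate, using a media map supplied by a MediaReader.
; Media player callbacks track loaded ID and play state and drive two timers.
; One timer auto-pauses playback after a set time; the other loops to broadcast seek time, duration and ID through the SeekFire dispatcher.
; Requests and callbacks report to an optional Logger.
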(event Custom|OpenFirstMedia
  ;[1 1 1] TESTING
  ; Events callable within the editor, used for testing purposes
  (bind _keys (Utilities|Map|Keys (Variables|Default|GetMediaMap)))
  (CallFunction|PlayMedia (Utilities|Array|Get(acopy) _keys) (Utilities|Struct|MakeMediaPlayerOptions "(Audio=0,Caption=-1,Metadata=-1,Script=-1,Subtitle=-1,Text=-1,Video=0)" (Math|Timespan|MakeTimespan 0 0 0 0 0) "Enabled" "Disabled")))

(event Custom|LoadMediaMap
  (bind _logger (Variables|Default|GetLogger))
  ;[1 1 1] INITIALISATION
  ; Events used for initialisation purposes of the module and binding to other modules
  ; to request data when it has been successfully created.
  (bind _mediareader (Variables|Default|GetMediaReader)
    (:then
      (bind _mediamap (Default|GetMediaMap _mediareader))
      (Variables|Default|SetMediaMap _mediamap)
      ;;[0.1686 1 0] Log: Media map successfully loaded
      (Utilities|IsValid _logger
        (:Is%20Valid
          (Default|Log _logger "MediaPlayer" "Log" "Media map successfully loaded" (Variables|Default|GetLog)))))
    (:else)))

(event Custom|EnableSeekFire
  ;[1 1 1] SEEKFIRE
  ; Events related to the broacasting of the media player seek position, media duration
  ; and media ID to other modules by using the event dispatcher along with the events
  ; for managing the timer handle.
  (bind _returnvalue (Utilities|Time|SetTimerbyFunctionName 0 "SendSeekInfo" (Variables|Default|GetFireInterval) true)))

(event Custom|OnSeekSet
  (bind _logger (Variables|Default|GetLogger))
  ;[1 1 1] MEDIAPLAYER REACTION EVENTS
  ; Events called as a response for the media player actions, these will determine what kind
  ; of action will be performed on the instant the media player opens, pauses, resumes... media
  ; playback, primarily used for logging purposes.
  ;;[0.1686 1 0] Log: Seek position updated
  (Utilities|IsValid _logger
    (:Is%20Valid
      (Default|Log _logger "MediaPlayer" "Log" "Seek position updated" (Variables|Default|GetLog)))))

(event Custom|OnResumed
  (bind _logger (Variables|Default|GetLogger))
  ;[1 1 1] MEDIAPLAYER REACTION EVENTS
  ; Events called as a response for the media player actions, these will determine what kind
  ; of action will be performed on the instant the media player opens, pauses, resumes... media
  ; playback, primarily used for logging purposes.
  (CallFunction|ResumeAutoPause)
  (CallFunction|ResumeSeekFire)
  (Variables|Default|SetIsPlaying true)
  ;;[0.1686 1 0] Log: Media playback resumed
  (Utilities|IsValid _logger
    (:Is%20Valid
      (Default|Log _logger "MediaPlayer" "Log" "Media playback resumed" (Variables|Default|GetLog)))))

(event Custom|SendSeekInfo
  ;[1 1 1] SEEKFIRE
  ; Events related to the broacasting of the media player seek position, media duration
  ; and media ID to other modules by using the event dispatcher along with the events
  ; for managing the timer handle.
  (bind _returnvalue (Class|MediaPlateComponent|GetMediaPlayer (Variables|Default|GetMediaPlateComponent)))
  (Default|CallSeekFire (Class|MediaPlayer|GetTime _returnvalue) (Media|MediaPlayer|GetDuration _returnvalue) (Variables|Default|GetLoadedMediaID) :!pinned true) ; Dispatch SeekFire with media data
)

(event Custom|PauseSeekFire
  ;[1 1 1] SEEKFIRE
  ; Events related to the broacasting of the media player seek position, media duration
  ; and media ID to other modules by using the event dispatcher along with the events
  ; for managing the timer handle.
  (Utilities|Time|PauseTimerbyHandle (stale Custom|EnableSeekFire _returnvalue)))

(event Custom|ResumeSeekFire
  ;[1 1 1] SEEKFIRE
  ; Events related to the broacasting of the media player seek position, media duration
  ; and media ID to other modules by using the event dispatcher along with the events
  ; for managing the timer handle.
  (Utilities|Time|UnpauseTimerbyHandle (stale Custom|EnableSeekFire _returnvalue)))

(event Custom|OnMediaOpen
  (params (OpenedUrl :type String))
  (bind _filenamepart (Utilities|String|Split OpenedUrl))
  (bind _logger (Variables|Default|GetLogger))
  ;[1 1 1] MEDIAPLAYER REACTION EVENTS
  ; Events called as a response for the media player actions, these will determine what kind
  ; of action will be performed on the instant the media player opens, pauses, resumes... media
  ; playback, primarily used for logging purposes.
  (Variables|Default|SetLoadedMediaID _filenamepart)
  (CallFunction|EnableSeekFire)
  ;;[0.1686 1 0] Log: Media playback resumed
  (Utilities|IsValid _logger
    (:Is%20Valid
      (Default|Log _logger "MediaPlayer" "Log" (Utilities|String|Append "Opened media with id: " _filenamepart) (Variables|Default|GetLog)))))

(event Custom|OnMediaFail
  (params (FailedUrl :type String))
  (bind _logger (Variables|Default|GetLogger))
  ;[1 1 1] MEDIAPLAYER REACTION EVENTS
  ; Events called as a response for the media player actions, these will determine what kind
  ; of action will be performed on the instant the media player opens, pauses, resumes... media
  ; playback, primarily used for logging purposes.
  (Media|MediaPlayer|Close (Variables|Default|GetMediaPlayer) :!class /Script/MediaAssets.MediaPlayer)
  (CallFunction|DisableSeekFire)
  (CallFunction|ClearAutoPause)
  (Variables|Default|SetLoadedMediaID "")
  (Variables|Default|SetIsPlaying false)
  ;;[1 0.1098 0] Error: Failed to open media
  (Utilities|IsValid _logger
    (:Is%20Valid
      (Default|Log _logger "MediaPlayer" "Error" (Utilities|String|Append "Failed to open media with id: " (.FilenamePart (Utilities|String|Split FailedUrl))) (Variables|Default|GetLog)))))

(event Custom|OnPaused
  (bind _logger (Variables|Default|GetLogger))
  ;[1 1 1] MEDIAPLAYER REACTION EVENTS
  ; Events called as a response for the media player actions, these will determine what kind
  ; of action will be performed on the instant the media player opens, pauses, resumes... media
  ; playback, primarily used for logging purposes.
  (CallFunction|PauseAutoPause)
  (CallFunction|PauseSeekFire)
  (Variables|Default|SetIsPlaying false)
  ;;[0.1686 1 0] Log media paused
  (Utilities|IsValid _logger
    (:Is%20Valid
      (Default|Log _logger "MediaPlayer" "Log" "Media playback paused" (Variables|Default|GetLog)))))

(event Custom|PauseMedia
  (bind _logger (Variables|Default|GetLogger))
  (bind _logger_2 (Variables|Default|GetLogger))
  ;[1 1 1] MEDIA PLAYER REQUEST EVENTS
  ; Events related to the request of an action to be executed by the media player, upon request
  ; the media player will be notified of the action to be executed and if possible it will be completed.
  ; Used for requesting a media to be played at a specific seek time, pausing and resuming the currently
  ; opened media.
  (Utilities|FlowControl|Sequence :!pinned true ; Request Pause
    (:then_0
      ;;[0.1686 1 0] Log: Pause media player request
      (Utilities|IsValid _logger
        (:Is%20Valid
          (Default|Log _logger "MediaPlayer" "Log" "Request | Pause playback" (Variables|Default|GetLog)))))
    (:then_1
      (bind _returnvalue (Sequencer|Player|Pause (Variables|Default|GetMediaPlayer)))
      (if (not _returnvalue)
        ;;[1 0.9098 0] Warning: Media player will not be paused
        (Utilities|IsValid _logger_2
          (:Is%20Valid
            (Default|Log _logger_2 "MediaPlayer" "Warning" "Request | Playback will not be paused" (Variables|Default|GetLog))))))))

(event Custom|ResumeMedia
  (bind _logger (Variables|Default|GetLogger))
  (bind _logger_2 (Variables|Default|GetLogger))
  ;[1 1 1] MEDIA PLAYER REQUEST EVENTS
  ; Events related to the request of an action to be executed by the media player, upon request
  ; the media player will be notified of the action to be executed and if possible it will be completed.
  ; Used for requesting a media to be played at a specific seek time, pausing and resuming the currently
  ; opened media.
  (Utilities|FlowControl|Sequence :!pinned true ; Request Resume
    (:then_0
      ;;[0.1686 1 0] Log: Resume media player request
      (Utilities|IsValid _logger
        (:Is%20Valid
          (Default|Log _logger "MediaPlayer" "Log" "Request | Resume playback" (Variables|Default|GetLog)))))
    (:then_1
      (bind _returnvalue (Media|MediaPlayer|Play (Variables|Default|GetMediaPlayer) :!class /Script/MediaAssets.MediaPlayer))
      (if (not _returnvalue)
        ;;[1 0.9098 0] Warning: Media player will not be resumed
        (Utilities|IsValid _logger_2
          (:Is%20Valid
            (Default|Log _logger_2 "MediaPlayer" "Warning" "Request | Playback will not be resumed" (Variables|Default|GetLog))))))))

(event Custom|PlayMedia
  (params (MediaID :type String%20%28by%20ref%29) (Options :type Media%20Player%20Options%20Structure%20%28by%20ref%29))
  (bind _logger (Variables|Default|GetLogger))
  (bind _mediamap (Variables|Default|GetMediaMap))
  (bind (_value _returnvalue) (Utilities|Map|Find _mediamap MediaID))
  ;[1 1 1] MEDIA PLAYER REQUEST EVENTS
  ; Events related to the request of an action to be executed by the media player, upon request
  ; the media player will be notified of the action to be executed and if possible it will be completed.
  ; Used for requesting a media to be played at a specific seek time, pausing and resuming the currently
  ; opened media.
  (Utilities|FlowControl|Sequence :!pinned true ; Request OpenSource
    (:then_1
      (if _returnvalue ; Find media id in media map
        (bind _returnvalue_2 (Media|MediaPlayer|OpenSourcewithOptions (Variables|Default|GetMediaPlayer) _value Options :!class /Script/MediaAssets.MediaPlayer))
        (if _returnvalue_2
          (CallFunction|ClearAutoPause)
          (CallFunction|PauseSeekFire)
          (else
            ;;[1 0.9098 0] Warning: Media will not be opened
            (Utilities|IsValid _logger :!label _label
              (:Is%20Valid
                (Default|Log _logger "MediaPlayer" "Warning" (Utilities|String|Append "Request | Cannot open media id: " MediaID) (Variables|Default|GetLog))))))
        (else
          (goto _label))))))

(event Custom|SetAutoPause
  (params (Time :type Float%20%28single-precision%29))
  ;[1 1 1] AUTOPAUSE
  ; Events related to the automatic pausing feature after a given amount of time
  ; along with the events for managing the timer handle.
  (bind _returnvalue (Utilities|Time|SetTimerbyFunctionName 0 "PauseMedia" Time)))

(event Custom|ClearAutoPause
  ;[1 1 1] AUTOPAUSE
  ; Events related to the automatic pausing feature after a given amount of time
  ; along with the events for managing the timer handle.
  (Utilities|Time|ClearandInvalidateTimerbyHandle (stale Custom|SetAutoPause _returnvalue)))

(event Custom|PauseAutoPause
  ;[1 1 1] AUTOPAUSE
  ; Events related to the automatic pausing feature after a given amount of time
  ; along with the events for managing the timer handle.
  (Utilities|Time|PauseTimerbyHandle (stale Custom|SetAutoPause _returnvalue)))

(event Custom|ResumeAutoPause
  ;[1 1 1] AUTOPAUSE
  ; Events related to the automatic pausing feature after a given amount of time
  ; along with the events for managing the timer handle.
  (Utilities|Time|UnpauseTimerbyHandle (stale Custom|SetAutoPause _returnvalue)))

(event Custom|DisableSeekFire
  ;[1 1 1] SEEKFIRE
  ; Events related to the broacasting of the media player seek position, media duration
  ; and media ID to other modules by using the event dispatcher along with the events
  ; for managing the timer handle.
  (Utilities|Time|ClearandInvalidateTimerbyHandle (stale Custom|EnableSeekFire _returnvalue)))

(event EventBeginPlay
  ;[1 1 1] INITIALISATION
  ; Events used for initialisation purposes of the module and binding to other modules
  ; to request data when it has been successfully created.
  (Utilities|FlowControl|Sequence
    (:then_0
      (bind _returnvalue (Class|MediaPlateComponent|GetMediaPlayer (Variables|Default|GetMediaPlateComponent)))
      (bind _output_get (Variables|Default|SetMediaPlayer _returnvalue))
      (Media|MediaSoundComponent|SetMediaPlayer (Variables|MediaPlate|GetMediaSound) _output_get) ; Update the MediaSound component to\nhave a reference to the media player
    )
    (:then_1
      (if (and (not (Utilities|IsValid (Variables|Default|GetLogger))) (Variables|Default|GetLog))
        (Development|PrintString "[Warning][MediaPlayer] Logging enabled but no Logger specified.")))
    (:then_2
      ;[1 1 1] MEDIAPLAYER REACTION EVENTS
      ; Events called as a response for the media player actions, these will determine what kind
      ; of action will be performed on the instant the media player opens, pauses, resumes... media
      ; playback, primarily used for logging purposes.
      (Utilities|FlowControl|Sequence :!pinned true ; Bind events to media player messages
        (:then_0
          (Media|MediaPlayer|BindEventtoOnMediaOpened (Variables|Default|GetMediaPlayer) (delegate Custom|OnMediaOpen) :!pinned true) ; OnMediaOpened
        )
        (:then_1
          (Media|MediaPlayer|BindEventtoOnMediaOpenFailed (Variables|Default|GetMediaPlayer) (delegate Custom|OnMediaFail) :!pinned true) ; OnMediaOpenFailed
        )
        (:then_2
          (EventDispatchers|BindEventtoOnSeekCompleted (Variables|Default|GetMediaPlayer) (delegate Custom|OnSeekSet) :!pinned true) ; OnSeekCompleted
        )
        (:then_3
          (Media|MediaPlayer|BindEventtoOnPlaybackResumed (Variables|Default|GetMediaPlayer) (delegate Custom|OnResumed) :!pinned true) ; OnPlaybackResumed
        )
        (:then_4
          (EventDispatchers|BindEventtoOnPlaybackSuspended (Variables|Default|GetMediaPlayer) (delegate Custom|OnPaused) :!pinned true) ; OnPlaybackSuspended
        )))
    (:then_3
      (bind _mediareader (Variables|Default|GetMediaReader :!pinned true) ; Bind LoadMediaMap to MediaReader\nMediaMapCreated event dispatcher
        (:then
          (EventDispatchers|BindEventtoMediaMapCreated _mediareader (delegate Custom|LoadMediaMap)))
        (:else
          (Development|PrintString "[Warning][MediaPlayer] MediaReader not specified."))))))

(fn ConstructionScript)

(fn GetMediaMap
  (return (Variables|Default|GetMediaMap)) ; Retrieve the media map within the media player
)

(fn GetPlayStatus
  (return (Variables|Default|GetIsPlaying)) ; Retrieve whether the mediaplate is playing a media
)