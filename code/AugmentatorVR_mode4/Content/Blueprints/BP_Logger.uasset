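; BP_Logger writes timestamped event messages and user action records, such as grab, teleport and match attempts, to two log files.
; Construction builds both paths from a full, project or content directory prefix; Initialise rebuilds them, but passes ActionLogFilePath as the action file name.
; Log rejects incomplete entries with a warning and appends bracketed lines if PrintToFile is set; its screen print is disconnected.
; LogAction always appends comma-separated rows when enabled, optionally printing them onscreen.
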(fn ConstructionScript
  (bind _filepath (CallFunction|ConstructPath (Variables|Default|GetPathType) (Variables|Default|GetPathPrefix) (Variables|Default|GetLogFileName)))
  (Variables|Default|SetLogFilePath _filepath)
  (bind _filepath_2 (CallFunction|ConstructPath (Variables|Default|GetPathType) (Variables|Default|GetPathPrefix) (Variables|Default|GetActionLogFileName)))
  (Variables|Default|SetActionLogFilePath _filepath_2))

(fn ConstructPath
  (params (PathType :type PathType%20Enum :default "NewEnumerator0") (Prefix :type String) (FileName :type String))
  (switch Utilities|FlowControl|Switch|SwitchonPathType PathType
    (:NewEnumerator0
      (return (Utilities|String|Append (Utilities|String|MakeLiteralString Prefix) FileName)))
    (:NewEnumerator1
      (return (Utilities|String|Append (Utilities|String|MakeLiteralString (Class|KismetSystemLibrary|GetProjectDirectory)) Prefix FileName)))
    (:NewEnumerator2
      (return (Utilities|String|Append (Utilities|String|MakeLiteralString (Class|KismetSystemLibrary|GetProjectContentDirectory)) Prefix FileName)))))

(fn ActiontoString
  (params (UserAction :type UserAction%20Enum :default "NewEnumerator0"))
  (switch Utilities|FlowControl|Switch|SwitchonUserAction UserAction
    (:NewEnumerator0
      (return "Grab"))
    (:NewEnumerator1
      (return "Release"))
    (:NewEnumerator2
      (return "Teleport"))
    (:NewEnumerator3
      (return "Touch"))
    (:NewEnumerator9
      (return "PlayAnnotation"))
    (:NewEnumerator10
      (return "Resume"))
    (:NewEnumerator11
      (return "Pause"))
    (:NewEnumerator14
      (return "CreateLinkStart"))
    (:NewEnumerator15
      (return "CreateLinkEnd"))
    (:NewEnumerator16
      (return "PlayVideo"))
    (:NewEnumerator17
      (return "MatchAttempt"))
    (:NewEnumerator19
      (return "ConceptSolve"))
    (:NewEnumerator20
      (return "ScoreSummary"))))

(fn GenerateTimestamp
  (bind _returnvalue (Math|DateTime|Now))
  (bind (_year _month _day _hour _minute _second _millisecond) (Math|DateTime|BreakDateTime _returnvalue))
  (return (Utilities|String|Append (Utilities|String|ToString(Integer) _year) "-" (Utilities|String|ToString(Integer) _month) "-" (Utilities|String|ToString(Integer) _day) "-" (Utilities|String|ToString(Integer) _hour) ":" (Utilities|String|ToString(Integer) _minute) ":" (Utilities|String|ToString(Integer) _second) ":" (Utilities|String|ToString(Integer) _millisecond))))

(fn Log
  (params (Module :type String) (Type :type String) (Message :type String) (Log :type Boolean))
  (bind _timestamp (CallFunction|GenerateTimestamp))
  (if Log
    (if (Math|Boolean|ORBoolean (Utilities|Array|IsEmpty Module) (Utilities|Array|IsEmpty Type) (Utilities|Array|IsEmpty Message))
      (CallFunction|Log "Logger" "Warning" "Could not log event because it was incomplete." true)
      (else
        (Utilities|FlowControl|Sequence
          (:then_0
            (if (Variables|Default|GetPrintToFile)
              (Class|FileSDKBPLibrary|WriteStringtoFile (Variables|Default|GetLogFilePath) (Utilities|String|Append "[" _timestamp "][" Module "][" Type "]:" Message " 
") true "AutoDetect")))
          (:then_1
            (if (Variables|Default|GetPrintToScreen)
              _)))))))

(fn LogAction
  (params (Log :type Boolean) (UserAction :type UserAction%20Enum :default "NewEnumerator0") (Data_1 :type String) (Data_2 :type String) (Data_3 :type String) (Data_4 :type String) (Data_5 :type String))
  (if Log
    (bind _timestamp (CallFunction|GenerateTimestamp))
    (bind _action (CallFunction|ActiontoString UserAction))
    (Utilities|FlowControl|Sequence
      (:then_0
        (Class|FileSDKBPLibrary|WriteStringtoFile (Variables|Default|GetActionLogFilePath) (Utilities|String|Append _timestamp "," _action "," Data_1 "," Data_2 "," Data_3 "," Data_4 "," Data_5 " 
") true "AutoDetect"))
      (:then_1
        (if (Variables|Default|GetPrintToScreen)
          (Development|PrintString (Utilities|String|Append _timestamp "," _action "," Data_1 "," Data_2 "," Data_3 "," Data_4 "," Data_5 " 
") true true "(R=0.963431,G=0.946885,B=1.000000,A=1.000000)" 1.2e+03))))))

(fn Initialise
  (bind _filepath (CallFunction|ConstructPath (Variables|Default|GetPathType) (Variables|Default|GetPathPrefix) (Variables|Default|GetLogFileName)))
  (Variables|Default|SetLogFilePath _filepath)
  (bind _filepath_2 (CallFunction|ConstructPath (Variables|Default|GetPathType) (Variables|Default|GetPathPrefix) (Variables|Default|GetActionLogFilePath)))
  (Variables|Default|SetActionLogFilePath _filepath_2))

(fn ConfigureParameters
  (params (LogFileName :type String) (ActionLogFileName :type String))
  (Utilities|FlowControl|Sequence
    (:then_0
      (Variables|Default|SetLogFileName LogFileName))
    (:then_1
      (Variables|Default|SetActionLogFileName ActionLogFileName))))