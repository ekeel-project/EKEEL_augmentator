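; BP_JsonReader is a data module actor that loads a JSON-LD graph of videos, concepts, prerequisite links and concept annotations.
; ReadJsonFile builds a configurable path, loads the file through VaRest and routes each "@graph" entry by type and motivation to a validating parser.
; Valid entries become structs in unique arrays exposed by getters, with timestamps converted to Timespans.
; An optional Logger records results, and ReadComplete fires one tick after parsing finishes.
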(event Custom|ReadJsonFile
  (bind _logger (Variables|Default|GetLogger))
  (bind _logger_2 (Variables|Default|GetLogger))
  (bind _logger_3 (Variables|Default|GetLogger))
  (bind _logger_4 (Variables|Default|GetLogger))
  (bind _logger_5 (Variables|Default|GetLogger))
  (bind _logger_6 (Variables|Default|GetLogger))
  (bind _logger_7 (Variables|Default|GetLogger))
  (bind _logger_8 (Variables|Default|GetLogger))
  (bind _logger_9 (Variables|Default|GetLogger))
  (bind _logger_10 (Variables|Default|GetLogger))
  (bind _logger_11 (Variables|Default|GetLogger))
  ;[1 1 1] FUNCTIONALITY
  ; Events related to the functionality of the module, executing the primary functions
  ; when required, typically bound to other modules to react and execute when data
  ; has been correctly instanced.
  (bind _filepath (CallFunction|ConstructPath (Variables|Default|GetPathType) (Variables|Default|GetPathPrefix) (Variables|Default|GetJsonFileName) :!pinned true)) ; Construct path
  (bind _returnvalue (Class|VaRestSubsystem|LoadJsonfromFile (|VaRestSubsystem) _filepath false :!pinned true)) ; Load Json File
  (Utilities|IsValid _returnvalue ; Start parsing if successfully read\nJson file
    (:Is%20Valid
      (Variables|Default|SetJsonFile _returnvalue)
      (Utilities|FlowControl|Sequence
        (:then_0
          ;;[0.1677 1 0] Log: Json file successfully loaded
          (Utilities|IsValid _logger_11
            (:Is%20Valid
              (Default|Log _logger_11 "JsonReader" "Log" "Json file successfully loaded." (Variables|Default|GetLog)))))
        (:then_1
          (Utilities|FlowControl|Sequence
            (:then_0
              (for _array_element (Class|VaRestJsonObject|GetObjectArrayField (Variables|Default|GetJsonFile) "@graph") ; Loop through the graph array within the Json file\neach entry will be distinguished and the appropriate\nparsing function will be called
                (switch string (Class|VaRestJsonObject|GetStringField _array_element "type")
                  (:Video
                    (bind (_valid _videodata) (CallFunction|ParseVideo _array_element :!pinned true)) ; Parse Video
                    (if _valid ; If parsing is successful add the video data\nto the array of valid data
                      (Utilities|Array|AddUnique (Variables|Default|GetVideos) _videodata)
                      ;;[0.1677 1 0] Log: Video entry successfully parsed
                      (Utilities|IsValid _logger_3
                        (:Is%20Valid
                          (Default|Log _logger_3 "JsonReader" "Log" (Utilities|String|Append "Video | added ID: " (Utilities|Struct|BreakS_Video _videodata)) (Variables|Default|GetLog))))
                      (else
                        ;;[1 0.9098 0] Warning: Could not parse Video entry
                        (Utilities|IsValid _logger_4
                          (:Is%20Valid
                            (Default|Log _logger_4 "JsonReader" "Warning" "Video | Could not read entry" (Variables|Default|GetLog)))))))
                  (:skos:Collection
                    (if (Utilities|Enum|Equal(Enum) (Class|VaRestJsonObject|GetStringField _array_element "id") "localVocabulary") ; Determine if the collection is\na local vocabulary containing concepts
                      (for _array_element_2 (Class|VaRestJsonObject|GetObjectArrayField _array_element "skos:member")
                        (bind (_valid_2 _conceptdata) (CallFunction|ParseConcept _array_element_2 :!pinned true)) ; Parse Concept
                        (if _valid_2 ; If parsing is successful add the concept data\nto the array of valid data
                          (Utilities|Array|AddUnique (Variables|Default|GetConcepts) _conceptdata)
                          ;;[0.1677 1 0] Log: Concept entry successfully parsed
                          (Utilities|IsValid _logger_9
                            (:Is%20Valid
                              (Default|Log _logger_9 "JsonReader" "Log" (Utilities|String|Append "Concept | added ID: " (.id (Utilities|Struct|BreakS_Concept _conceptdata))) (Variables|Default|GetLog))))
                          (else
                            ;;[1 0.9098 0] Warning: Could not parse Concept entry
                            (Utilities|IsValid _logger_6
                              (:Is%20Valid
                                (Default|Log _logger_6 "JsonReader" "Warning" "Concept | Could not read entry" (Variables|Default|GetLog)))))))))
                  (:Annotation
                    (switch string (Class|VaRestJsonObject|GetStringField _array_element "motivation") ; Determine if the annotation type represents\na link or a concept definition
                      (:edu:linkingPrerequisite
                        (bind (_valid_3 _linkdata) (CallFunction|ParseLink _array_element :!pinned true)) ; Parse Link
                        (if _valid_3 ; If parsing is successful add the link data\nto the array of valid data
                          (Utilities|Array|AddUnique (Variables|Default|GetLinks) _linkdata)
                          ;;[0.1677 1 0] Log: Link entry successfully parsed
                          (Utilities|IsValid _logger_10
                            (:Is%20Valid
                              (Default|Log _logger_10 "JsonReader" "Log" (Utilities|String|Append "Link | added ID: " (.link_id (Utilities|Struct|BreakS_Link _linkdata))) (Variables|Default|GetLog))))
                          (else
                            ;;[1 0.9098 0] Warning: Could not parse Link entry
                            (Utilities|IsValid _logger_8
                              (:Is%20Valid
                                (Default|Log _logger_8 "JsonReader" "Warning" "Link | Could not read entry" (Variables|Default|GetLog)))))))
                      (:describing
                        (bind (_valid_4 _conceptannotationdata) (CallFunction|ParseConceptAnnotation _array_element :!pinned true)) ; Parse ConceptAnnotation
                        (if _valid_4 ; If parsing is successful add the concept annotation data\nto the array of valid data
                          (Utilities|Array|AddUnique (Variables|Default|GetAnnotations) _conceptannotationdata)
                          ;;[0.1677 1 0] Log: ConceptAnnotation entry successfully parsed
                          (Utilities|IsValid _logger_2
                            (:Is%20Valid
                              (Default|Log _logger_2 "JsonReader" "Log" (Utilities|String|Append "Annotation | added ID: " (.ann_id (Utilities|Struct|BreakS_ConceptAnnotation _conceptannotationdata))) (Variables|Default|GetLog))))
                          (else
                            ;;[1 0.9098 0] Warning: Could not parse ConceptAnnotation entry
                            (Utilities|IsValid _logger
                              (:Is%20Valid
                                (Default|Log _logger "JsonReader" "Warning" "Annotation | Could not read entry" (Variables|Default|GetLog))))))))))))
            (:then_1
              (Utilities|FlowControl|Sequence :!pinned true ; Dispatch ReadComplete
                (:then_0
                  ;;[0.1677 1 0] Log: Completed parsing Json file
                  (Utilities|IsValid _logger_5
                    (:Is%20Valid
                      (Default|Log _logger_5 "JsonReader" "Log" "Completed json parsing, calling ReadComplete" (Variables|Default|GetLog)))))
                (:then_1
                  (Utilities|FlowControl|DelayUntilNextTick)
                  (Default|CallReadComplete))))))))
    (:Is%20Not%20Valid
      (Utilities|FlowControl|Sequence
        (:then_0
          ;;[1 0.1083 0] Error: Could not read Json file
          (Utilities|IsValid _logger_7
            (:Is%20Valid
              (Default|Log _logger_7 "JsonReader" "Error" " Could not read json file." (Variables|Default|GetLog)))))
        (:then_1
          (Development|PrintString "Could not read json file."))))))

(event EventBeginPlay
  ;[1 1 1] INITIALISATION
  ; Initialisation events that set up the module variables and bind events to other
  ; connected modules if present.
  (if (not (not (and (not (Utilities|IsValid (Variables|Default|GetLogger))) (Variables|Default|GetLog))))
    (Development|PrintString "[Warning][JsonReader] Logging enabled but no Logger specified.")))

(fn ConstructionScript)

(fn GetConcepts
  (return (Variables|Default|GetConcepts)) ; Returns the array of successfully parsed concept data
)

(fn GetLinks
  (return (Variables|Default|GetLinks)) ; Returns the array of successfully parsed link data
)

(fn GetAnnotations
  (return (Variables|Default|GetAnnotations)) ; Returns the array of successfully parsed annotation data
)

(fn GetVideos
  (return (Variables|Default|GetVideos)) ; Returns the array of successfully parsed video data
)

(fn ParseTimeString
  (params (TimeString :type String))
  (bind _returnvalue (Utilities|String|MakeLiteralString "^^xsd:dateTime"))
  (bind _lefts (Utilities|String|Split TimeString _returnvalue "CaseSensitive" "FromEnd"))
  (bind (_result _returnvalue_2) (Class|KismetMathLibrary|TimespanfromString _lefts))
  (return _returnvalue_2 _result))

(fn ParseVideo
  (params (VideoEntry :type Va%20Rest%20Json%20Object%20Object%20Reference))
  (bind _returnvalue (Class|VaRestJsonObject|GetStringField VideoEntry "id"))
  (if (Utilities|Enum|Equal(Enum) (Class|VaRestJsonObject|GetStringField VideoEntry "type") "Video") ; Check if entry given is a video entry
    ;[1 1 1] Validate and create S_Video structure
    (if (not (Utilities|Array|IsEmpty _returnvalue)) ; Validate\nAll fields must exist
      (return true (Utilities|Struct|MakeS_Video _returnvalue))
      (else
        _)))
  (return false ""))

(fn ParseConcept
  (params (ConceptEntry :type Va%20Rest%20Json%20Object%20Object%20Reference))
  (bind _returnvalue (Class|VaRestJsonObject|GetObjectField ConceptEntry "skos:prefLabel"))
  (bind _returnvalue_2 (Class|VaRestJsonObject|GetStringField ConceptEntry "id"))
  (bind _returnvalue_3 (Class|VaRestJsonObject|GetStringField _returnvalue "@value"))
  (if (Utilities|Enum|Equal(Enum) (Class|VaRestJsonObject|GetStringField ConceptEntry "type") "skos:Concept") ; Check if entry given is a concept entry
    ;[1 1 1] Validate and create S_Concept structure
    (if (and (not (Utilities|Array|IsEmpty _returnvalue_2)) (not (Utilities|Array|IsEmpty _returnvalue_3))) ; Validate\nAll fields must exist
      (return true (Utilities|Struct|MakeS_Concept _returnvalue_2 _returnvalue_3))
      (else
        _)))
  (return false ""))

(fn ParseConceptAnnotation
  (params (ConceptAnnotationEntry :type Va%20Rest%20Json%20Object%20Object%20Reference))
  (bind _returnvalue (Class|VaRestJsonObject|GetStringField ConceptAnnotationEntry "body"))
  (bind _returnvalue_2 (Class|VaRestJsonObject|GetStringField ConceptAnnotationEntry "motivation"))
  (bind _returnvalue_3 (Class|VaRestJsonObject|GetStringField ConceptAnnotationEntry "skos:note"))
  (bind _returnvalue_4 (Class|VaRestJsonObject|GetStringField ConceptAnnotationEntry "id"))
  (bind _returnvalue_5 (Class|VaRestJsonObject|GetObjectField ConceptAnnotationEntry "target"))
  (bind _returnvalue_6 (Class|VaRestJsonObject|GetStringField _returnvalue_5 "source"))
  (bind _returnvalue_7 (Class|VaRestJsonObject|GetObjectField _returnvalue_5 "selector"))
  (if (and (Utilities|Enum|Equal(Enum) (Class|VaRestJsonObject|GetStringField ConceptAnnotationEntry "type") "Annotation") (Utilities|Enum|Equal(Enum) (Class|VaRestJsonObject|GetStringField ConceptAnnotationEntry "motivation") "describing")) ; Check if entry given is a concept annotation entry\n(Annotation + Describing)
    ;[1 1 1] Validate and create S_ConceptAnnotation structure
    (Utilities|FlowControl|Sequence ; Parse the timestamps first
      (:then_0
        (bind (_valid _timespan) (CallFunction|ParseTimeString (Class|VaRestJsonObject|GetStringField (Class|VaRestJsonObject|GetObjectField _returnvalue_7 "startSelector") "value"))))
      (:then_1
        (bind (_valid_2 _timespan_2) (CallFunction|ParseTimeString (Class|VaRestJsonObject|GetStringField (Class|VaRestJsonObject|GetObjectField _returnvalue_7 "endSelector") "value"))))
      (:then_2
        (if (Math|Boolean|ANDBoolean (not (Utilities|Array|IsEmpty _returnvalue)) (not (Utilities|Array|IsEmpty _returnvalue_4)) (not (Utilities|Array|IsEmpty _returnvalue_2)) (not (Utilities|Array|IsEmpty _returnvalue_3)) (not (Utilities|Array|IsEmpty _returnvalue_6)) _valid _valid_2) ; Validate\nAll fields must exist
          (return true (Utilities|Struct|MakeS_ConceptAnnotation _returnvalue _returnvalue_4 _returnvalue_2 _returnvalue_3 _returnvalue_6 _timespan _timespan_2))
          (else
            (return false "")))))
    (else
      (return false ""))))

(fn ParseLink
  (params (LinkEntry :type Va%20Rest%20Json%20Object%20Object%20Reference))
  (bind _returnvalue (Class|VaRestJsonObject|GetObjectField LinkEntry "target"))
  (bind _returnvalue_2 (Class|VaRestJsonObject|GetStringField LinkEntry "motivation"))
  (bind _returnvalue_3 (Class|VaRestJsonObject|GetStringField LinkEntry "skos:note"))
  (bind _returnvalue_4 (Class|VaRestJsonObject|GetStringField LinkEntry "id"))
  (bind _returnvalue_5 (Class|VaRestJsonObject|GetStringField LinkEntry "body"))
  (bind _returnvalue_6 (Class|VaRestJsonObject|GetObjectField _returnvalue "dcterms:subject"))
  (bind _returnvalue_7 (Class|VaRestJsonObject|GetStringField _returnvalue "source"))
  (bind _returnvalue_8 (Class|VaRestJsonObject|GetStringField _returnvalue_6 "id"))
  (if (and (Utilities|Enum|Equal(Enum) (Class|VaRestJsonObject|GetStringField LinkEntry "type") "Annotation") (Utilities|Enum|Equal(Enum) (Class|VaRestJsonObject|GetStringField LinkEntry "motivation") "edu:linkingPrerequisite")) ; Check if entry given is a link entry\n(Annotation + LinkingPrerequisite)
    ;[1 1 1] Validate and create S_Link structure
    (Utilities|FlowControl|Sequence
      (:then_0
        (bind (_valid _timespan) (CallFunction|ParseTimeString (Class|VaRestJsonObject|GetStringField (Class|VaRestJsonObject|GetObjectField _returnvalue "selector") "value"))))
      (:then_1
        (if (Math|Boolean|ANDBoolean (not (Utilities|Array|IsEmpty _returnvalue_5)) (not (Utilities|Array|IsEmpty _returnvalue_8)) (not (Utilities|Array|IsEmpty _returnvalue_4)) (not (Utilities|Array|IsEmpty _returnvalue_2)) (not (Utilities|Array|IsEmpty _returnvalue_3)) (not (Utilities|Array|IsEmpty _returnvalue_7)) _valid) ; Validate\nAll fields must exist
          (return true (Utilities|Struct|MakeS_Link _returnvalue_5 _returnvalue_8 _returnvalue_4 _returnvalue_2 _returnvalue_3 _returnvalue_7 (Utilities|String|Append "name_" (Class|VaRestJsonObject|GetStringField LinkEntry "id")) _timespan))
          (else
            (return false "")))))
    (else
      (return false ""))))

(fn ConstructPath
  (params (PathType :type PathType%20Enum :default "NewEnumerator0") (Prefix :type String) (FileName :type String))
  (switch Utilities|FlowControl|Switch|SwitchonPathType PathType
    (:NewEnumerator0
      (return (Utilities|String|Append (Utilities|String|MakeLiteralString Prefix) FileName)))
    (:NewEnumerator1
      (return (Utilities|String|Append (Utilities|String|MakeLiteralString (Class|KismetSystemLibrary|GetProjectDirectory)) Prefix FileName)))
    (:NewEnumerator2
      (return (Utilities|String|Append (Utilities|String|MakeLiteralString (Class|KismetSystemLibrary|GetProjectContentDirectory)) Prefix FileName)))))

(fn ConfigureParameters
  (params (JsonFileName :type String))
  (Variables|Default|SetJsonFileName JsonFileName))