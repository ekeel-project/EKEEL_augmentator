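; BP_Configurator is the startup hub that configures the simulation's connected modules for one of four modes.
; On BeginPlay it validates each reference in sequence, warning if missing, and passes Mode-selected flags to the Spawner, VRCharacter and HighlighterVisualiser.
; It also initialises the Logger with file names, sets the Spawner's glass-sphere percentage regardless of mode, and starts the JsonReader's file read last.
; Delayed-sound and timestamped-filename nodes are left unconnected.
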(event EventBeginPlay
  (bind _mode (Variables|Default|GetMode))
  (bind _returnvalue (Utilities|Select :Index _mode :NewEnumerator0 false :NewEnumerator1 false :NewEnumerator2 false :NewEnumerator3 true))
  ;[0 0 0] INITIALISATION
  ; Events used for initialisation purposes of the module and configuration of the
  ; connected modules..
  ;;[1 1 1] BEGIN PLAY
  (Utilities|FlowControl|Sequence
    (:then_0
      (bind _logger (Variables|Default|GetLogger :!pinned true) ; Logger
        (:then
          (Default|ConfigureParameters _logger (Variables|Default|GetLog%20File%20Name) (Variables|Default|GetAction%20Log%20File%20Name))
          (Default|Initialise _logger))
        (:else
          (Development|PrintString "[Warning][Configurator] Logger not specified."))))
    (:then_1
      (bind _spawner (Variables|Default|GetSpawner :!pinned true) ; Spawner
        (:then
          (Default|ConfigureParameters _spawner (Utilities|Select :Index (Variables|Default|GetMode) :NewEnumerator0 false :NewEnumerator1 true :NewEnumerator2 false :NewEnumerator3 false) (Utilities|Select :Index (Variables|Default|GetMode) :NewEnumerator0 false :NewEnumerator1 true :NewEnumerator2 true :NewEnumerator3 false) (Utilities|Select :Index (Variables|Default|GetMode) :NewEnumerator0 false :NewEnumerator1 true :NewEnumerator2 false :NewEnumerator3 false) false)
          (Variables|Default|SetSelectedOption _returnvalue)
          (Variables|Default|SetIsModeFour _returnvalue)
          ;[0.5885 0.5748 0.5809] Imposta la percentuale di sfere di vetro del Mode Four
          (Variables|/Game/Blueprints/BP_Spawner.BP_Spawner_C|SetGlassSpherePercentage (Variables|Default|GetSpawner) 99.0))
        (:else
          (Development|PrintString "[Warning][Configurator] Spawner not specified."))))
    (:then_2
      (bind _vrcharacter (Variables|Default|GetVRCharacter :!pinned true) ; VRCHaracter
        (:then
          (Default|ConfigureParameters _vrcharacter (Utilities|Select :Index (Variables|Default|GetMode) :NewEnumerator0 false :NewEnumerator1 false :NewEnumerator2 true :NewEnumerator3 false)))
        (:else
          (Development|PrintString "[Warning][Configurator] VRCharacrer not specified."))))
    (:then_3
      (bind _highlightervisualiser (Variables|Default|GetHighlighterVisualiser :!pinned true) ; HighlighterVisualiser
        (:then
          (Default|ConfigureParameters _highlightervisualiser (Utilities|Select :Index (Variables|Default|GetMode) :NewEnumerator0 true :NewEnumerator1 true :NewEnumerator2 true :NewEnumerator3 false) (Utilities|Select :Index (Variables|Default|GetMode) :NewEnumerator0 false :NewEnumerator1 true :NewEnumerator2 false :NewEnumerator3 false)))
        (:else
          (Development|PrintString "[Warning][Configurator] HighlighterVisualiser not specified."))))
    (:then_4
      (bind _jsonreader (Variables|Default|GetJsonReader :!pinned true) ; JsonReader
        (:then
          (Default|ConfigureParameters _jsonreader (Variables|Default|GetJson%20File%20Name))
          (Default|ReadJsonFile _jsonreader :!pinned true) ; Initiate reading operation
        )
        (:else
          (Development|PrintString "[Warning][Configurator] JsonReader not specified."))))))

(fn ConstructionScript)