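; Spawner module that builds concept spheres, links and annotations from JsonReader data once reading completes.
; It spawns a table row of concepts, plus map copies if BP_Configurator's option is set, which replace them in the ID map used by links and annotations.
; Mapped concepts are arranged by first mention, total mentions and a triangle wave.
; Mode Four turns random map spheres into unlabelled "glass", keeping only their table twins, matched by actor-name index.
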(event Custom|Spawn
  (bind _logger (Variables|Default|GetLogger))
  (bind _logger_2 (Variables|Default|GetLogger))
  (bind _logger_3 (Variables|Default|GetLogger))
  (bind _logger_4 (Variables|Default|GetLogger))
  (bind _logger_5 (Variables|Default|GetLogger))
  (bind _logger_6 (Variables|Default|GetLogger))
  (bind _logger_7 (Variables|Default|GetLogger))
  (bind _logger_8 (Variables|Default|GetLogger))
  (bind _filteredmapspheresarray (Variables|Default|GetFilteredMapSpheresArray))
  (bind _spawnedtablespheres (Variables|Default|GetSpawnedTableSpheres))
  (bind _logger_9 (Variables|Default|GetLogger))
  ;[1 1 1] Events related to the primary function of the Spawner module which will
  ; generate the concepts, links and annotations using the parameters of
  ; the spawner and log the results if logging is enabled.
  ;;[1 1 1] Events used for initialisation purposes of the module and binding to other modules
  ;; to request data when it has been successfully created.
  (Utilities|FlowControl|Sequence
    (:then_0
      (if (Variables|Default|GetSpawnConcepts)
        (bind _jsonreader (Variables|Default|GetJsonReader)
          (:then
            (bind _concepts (Default|GetConcepts _jsonreader))
            (for _array_element _concepts ; Try spawning all concepts
              (bind (_valid _concept) (CallFunction|SpawnConcept _array_element))
              (Utilities|FlowControl|Sequence
                (:then_0
                  (Utilities|FlowControl|Sequence
                    (:then_0
                      (if _valid
                        (Utilities|Map|Add (Variables|Default|GetConceptActors) (.id (Utilities|Struct|BreakS_Concept _array_element)) _concept)
                        ;;[0.1677 1 0] Log: Concept actor successfully spawned
                        (Utilities|IsValid _logger_7
                          (:Is%20Valid
                            (Default|Log _logger_7 "Spawner" "Log" (Utilities|String|Append "Concept | added ID: " (.id (Utilities|Struct|BreakS_Concept _array_element))) (Variables|Default|GetLog))))
                        (else
                          ;;[1 0.9098 0] Warning: Could not spawn concept actor
                          (Utilities|IsValid _logger_8
                            (:Is%20Valid
                              (Default|Log _logger_8 "Spawner" "Warning" "Concept | Could not spawn actor" (Variables|Default|GetLog)))))))))
                (:then_1
                  (Utilities|Array|Add _spawnedtablespheres _concept)
                  (for _array_element_2 _spawnedtablespheres
                    (bind _asbp_concept (Utilities|Casting|CastToBP_Concept _array_element_2))))))
            (for _array_element_3 _concepts
              ;;[0.1677 1 0] Create reference from  BP_Configurator and retrieves variable SelectedOption's value
              (bind _outactors (Actor|GetAllActorsOfClass "/Game/Blueprints/BP_Configurator.BP_Configurator_C"))
              (if (Variables|/Game/Blueprints/BP_Configurator.BP_Configurator_C|GetSelectedOption (Utilities|Array|Get(acopy) _outactors))
                (bind _concept_2 (CallFunction|SpawnConceptB _array_element_3))
                (Variables|/Game/Blueprints/BP_Concept.BP_Concept_C|SetIsMapSphere _concept_2 true)
                (if true
                  (Utilities|Map|Add (Variables|Default|GetConceptActors) (.id (Utilities|Struct|BreakS_Concept _array_element_3)) _concept_2)
                  ;[0.1677 1 0] Log: Concept actor successfully spawned
                  (Utilities|IsValid _logger
                    (:Is%20Valid
                      (Default|Log _logger "Spawner" "Log" (Utilities|String|Append "Concept | added ID: " (.id (Utilities|Struct|BreakS_Concept _array_element_3))) (Variables|Default|GetLog))))
                  (else
                    ;[1 0.9098 0] Warning: Could not spawn concept actor
                    (Utilities|IsValid _logger_2
                      (:Is%20Valid
                        (Default|Log _logger_2 "Spawner" "Warning" "Concept | Could not spawn actor" (Variables|Default|GetLog)))))))))
          (:else))))
    (:then_1
      (if (Variables|Default|GetSpawnLinks)
        (bind _jsonreader_2 (Variables|Default|GetJsonReader)
          (:then
            (bind _links (Default|GetLinks _jsonreader_2))
            (for _array_element_4 _links ; Try spawning all links
              (bind (_valid_2 _link) (CallFunction|SpawnLink _array_element_4))
              (if _valid_2
                (Utilities|Map|Add (Variables|Default|GetLinkActors) (.link_id (Utilities|Struct|BreakS_Link _array_element_4)) _link)
                ;;[0.1677 1 0] Log: Link actor successfully spawned
                (Utilities|IsValid _logger_3
                  (:Is%20Valid
                    (Default|Log _logger_3 "Spawner" "Log" (Utilities|String|Append "Link | added ID: " (.link_id (Utilities|Struct|BreakS_Link _array_element_4))) (Variables|Default|GetLog))))
                (else
                  ;;[1 0.9098 0] Warning: Could not spawn link actor
                  (Utilities|IsValid _logger_4
                    (:Is%20Valid
                      (Default|Log _logger_4 "Spawner" "Warning" "Link | Could not spawn actor" (Variables|Default|GetLog))))))))
          (:else))))
    (:then_2
      (if (Variables|Default|GetLoadAnnotations)
        (bind _jsonreader_3 (Variables|Default|GetJsonReader)
          (:then
            (bind _annotations (Default|GetAnnotations _jsonreader_3))
            (for _array_element_5 _annotations ; Try adding all annotations
              (bind _valid_3 (CallFunction|LoadAnnotation _array_element_5))
              (if _valid_3
                ;;[0.1677 1 0] Log: Annotation successfully added
                (Utilities|IsValid _logger_9
                  (:Is%20Valid
                    (Default|Log _logger_9 "Spawner" "Log" (Utilities|String|Append "Annotation | added ID: " (.ann_id (Utilities|Struct|BreakS_ConceptAnnotation _array_element_5))) (Variables|Default|GetLog))))
                (else
                  ;;[1 0.9098 0] Warning: Could not add annotation
                  (Utilities|IsValid _logger_6
                    (:Is%20Valid
                      (Default|Log _logger_6 "Spawner" "Warning" "Annotation | Could not add annotation" (Variables|Default|GetLog))))))))
          (:else))))
    (:then_3
      (CallFunction|RepositionConcepts :!pinned true) ; Reposition Concepts
    )
    (:then_4
      (CallFunction|RepositionConceptsB))
    (:then_5
      (Utilities|FlowControl|Sequence :!pinned true ; Dispatch SpawnComplete
        (:then_0
          ;;[0.1677 1 0] Log: Completed spawning operation
          (Utilities|IsValid _logger_5
            (:Is%20Valid
              (Default|Log _logger_5 "Spawner" "Log" "Completed spawning actors, calling SpawnComplete" (Variables|Default|GetLog)))))
        (:then_1
          (Utilities|FlowControl|DelayUntilNextTick)
          (Default|CallSpawnComplete)
          ;;[1 1 1] 1_Recupera la variabile IsModeFour per le logiche successive del Mode Four
          (bind _outactors_2 (Actor|GetAllActorsOfClass "/Game/Blueprints/BP_Configurator.BP_Configurator_C"))
          (if (Variables|/Game/Blueprints/BP_Configurator.BP_Configurator_C|GetIsModeFour (Utilities|Array|Get(acopy) _outactors_2))
            ;;[1 1 1] 2_Memorizza in un array l'elenco delle sfere della mappa
            (bind _outactors_3 (Actor|GetAllActorsOfClass "/Game/Blueprints/BP_Concept.BP_Concept_C"))
            (for _array_element_6 _outactors_3
              (bind _asbp_concept_2 (Utilities|Casting|CastToBP_Concept _array_element_6))
              (if (Variables|/Game/Blueprints/BP_Concept.BP_Concept_C|GetIsMapSphere _asbp_concept_2)
                (Utilities|Array|Add _filteredmapspheresarray _asbp_concept_2)))
            (Variables|Default|SetMapSpawnedSpheres (Utilities|Array|Length _filteredmapspheresarray))
            ;[1 1 1] 4_Calcola la quantità di sfere di vetro nella mappa, basata sulla variabile GlassSpherePercentage nel Configurator
            (Variables|Default|SetGlassSpheresCount (Math|Float|Ceil (/ (* (Utilities|Array|Length (Variables|Default|GetFilteredMapSpheresArray)) (Variables|Default|GetGlassSpherePercentage)) 1e+02)))
            ;[1 1 1] 5_Rimescola le sfere nell'array della mappa e ne inserisce il GlassSpherePercentage % nell'array SelectedGlassSpheres
            (Utilities|Array|Shuffle (Variables|Default|GetFilteredMapSpheresArray))
            (Utilities|Array|Clear (Variables|Default|GetSelectedGlassSpheres))
            (for _index (range 0 (- (Variables|Default|GetGlassSpheresCount) 1))
              (Utilities|Array|Add (Variables|Default|GetSelectedGlassSpheres) (Utilities|Array|Get(acopy) (Variables|Default|GetFilteredMapSpheresArray) _index)))
            (for _array_element_7 (Variables|Default|GetSelectedGlassSpheres)
              (bind _asbp_concept_3 (Utilities|Casting|CastToBP_Concept _array_element_7))
              ;[1 1 1] Trasforma i nomi delle SelectedGlassSpheres nella mappa in un array di stringhe ValidTableSpheresNames
              (Utilities|Array|Add (Variables|Default|GetValidTableSphereNames) (Utilities|String|Append "BP_Concept_C_" (Utilities|String|ToString(Integer) (- (Math|Conversions|ToInteger(Byte) (Utilities|String|RightChop (Utilities|GetDisplayName _asbp_concept_3) 13)) (Variables|Default|GetMapSpawnedSpheres))))))
            (Utilities|FlowControl|Sequence
              (:then_0
                ;[1 1 1] Trasforma l'array di stringhe ValidTableSpheresNames nell'array ValidTableSpheres
                (bind _outactors_4 (Actor|GetAllActorsOfClass "/Game/Blueprints/BP_Concept.BP_Concept_C"))
                (for _array_element_8 _outactors_4
                  (if (Utilities|Array|ContainsItem (Variables|Default|GetValidTableSphereNames) (Utilities|GetDisplayName _array_element_8))
                    (Utilities|Array|Add (Variables|Default|GetValidTableSpheres) _array_element_8))))
              (:then_1
                ;[1 1 1] 6_Per le sfere dell'array SlectedGlassSpheres imposta a True la variabile IsGlassSphere
                (for _array_element_9 (Variables|Default|GetSelectedGlassSpheres)
                  (bind _asbp_concept_4 (Utilities|Casting|CastToBP_Concept _array_element_9))
                  (Variables|/Game/Blueprints/BP_Concept.BP_Concept_C|SetIsGlassSphere _asbp_concept_4 true))
                ;[1 1 1] 8_Imposta il parametro Base delle sfere di vetro e nasconde le etichette
                (for _array_element_10 (Variables|Default|GetSelectedGlassSpheres)
                  (bind _asbp_concept_5 (Utilities|Casting|CastToBP_Concept _array_element_10))
                  (if (Variables|/Game/Blueprints/BP_Concept.BP_Concept_C|GetIsGlassSphere _asbp_concept_5)
                    (Rendering|Material|SetVectorParameterValueonMaterials (Variables|/Game/Blueprints/BP_Concept.BP_Concept_C|GetStaticMesh _asbp_concept_5) "Base" "1.000000,0.990000,0.000000")
                    (bind _output_get (Variables|Default|SetNew%20Visibility false))
                    ;[1 1 1] 7_Per le sfere dell'array SlectedGlassSpheres salva materiale ed etichetta in due variabili del bp_concept
                    (Rendering|SetVisibility (Variables|/Game/Blueprints/BP_Concept.BP_Concept_C|GetWidgetLabel _asbp_concept_5) _output_get false)))
                ;[1 1 1] Elimina le sfere non necessarie dal tavolino
                (for _array_element_11 (Variables|Default|GetSpawnedTableSpheres)
                  (if (not (Utilities|Array|ContainsItem (Variables|Default|GetValidTableSpheres) _array_element_11))
                    (Utilities|IsValid _array_element_11
                      (:Is%20Valid
                        (Actor|DestroyActor _array_element_11)))))))))))))

(event EventBeginPlay
  ;[1 1 1] Events used for initialisation purposes of the module and binding to other modules
  ; to request data when it has been successfully created.
  (Utilities|FlowControl|Sequence
    (:then_0
      (if (and (not (Utilities|IsValid (Variables|Default|GetLogger))) (Variables|Default|GetLog))
        (Development|PrintString "[Warning][Spawner] Logging enabled but no Logger specified.")))
    (:then_1
      (Variables|Default|GetAnnotationMenu
        (:then)
        (:else
          (Development|PrintString "[Warning][Spawner] AnnotationMenu not specified."))))
    (:then_2
      (bind _jsonreader (Variables|Default|GetJsonReader :!pinned true) ; Bind Spawn to JsonReader\nReadComplete dispatcher
        (:then
          (EventDispatchers|BindEventtoReadComplete _jsonreader (delegate Custom|Spawn)))
        (:else
          (Development|PrintString "[Warning][Spawner] JsonReader not specified."))))))

(fn ConstructionScript)

(fn GetConceptActorMap
  (return (Variables|Default|GetConceptActors)) ; Returns the generated concept actors
)

(fn GetLinkActorMap
  (return (Variables|Default|GetLinkActors)) ; Returns the generated link actors
)

(fn SpawnConcept
  (params (ConceptData :type S%20Concept%20Structure))
  (Variables|Default|SetSpawnIndex (+ (Variables|Default|GetSpawnIndex) 1))
  (bind _returnvalue (Game|SpawnActorfromClass "/Game/Blueprints/BP_Concept.BP_Concept_C" (Math|Transform|MakeTransform (+ (.Origin (Collision|GetComponentBounds (select (Variables|Default|GetUseSecondaryBox) (Variables|Default|GetSecondaryBox) (Variables|Default|GetTertiaryBox)))) (* (Variables|Default|GetSpawnOffset) (Variables|Default|GetSpawnIndex))) "0, 0, 0" (Math|Conversions|ToVector(Float) (Variables|Default|GetConceptScale))) "AlwaysSpawn" "MultiplyWithRoot" 0 0 :!pinned true)) ; Spawn concept actor
  ;[1 1 1] Initialise concept actor with data
  (Default|SetConceptData _returnvalue ConceptData)
  (Default|SetAnnotationMenu _returnvalue (Variables|Default|GetAnnotationMenu))
  (Default|SetVisibility _returnvalue (not (Variables|Default|GetHideConcepts)))
  (return true _returnvalue))

(fn SpawnLink
  (params (LinkData :type S%20Link%20Structure))
  (bind _conceptactors (Variables|Default|GetConceptActors))
  (bind (_start_concept_id _end_concept_id) (Utilities|Struct|BreakS_Link LinkData))
  (bind (_value _returnvalue) (Utilities|Map|Find _conceptactors _start_concept_id))
  (bind (_value_2 _returnvalue_2) (Utilities|Map|Find _conceptactors _end_concept_id))
  (if (and _returnvalue _returnvalue_2) ; If concept end points are\nmissing avoid spawning
    (bind _returnvalue_3 (Game|SpawnActorfromClass "/Game/Blueprints/BP_Link.BP_Link_C" (Math|Transform|MakeTransform "0, 0, 0" "0, 0, 0" (Math|Conversions|ToVector(Float) (Variables|Default|GetLinkScale))) "Undefined" "MultiplyWithRoot" 0 0 :!pinned true)) ; Spawn link actor
    ;[1 1 1] Initialise link actor with data
    (Default|SetLinkData _returnvalue_3 LinkData)
    (Default|SetLinkColour _returnvalue_3 (Variables|Default|GetLinkColour))
    (Default|SetLabelVisibility _returnvalue_3 (Variables|Default|GetLinkLabels))
    (Default|SetVisibility _returnvalue_3 (not (Variables|Default|GetHideLinks)))
    (Default|SetEndActor _returnvalue_3 _value_2) ; Set end point
    (bind _returnvalue_4 (Transformation|AttachActorToActor _returnvalue_3 _value "None" "KeepRelative" "KeepWorld" "KeepWorld" false)) ; Set start point by attaching to another actor
    (if _returnvalue_4
      (return true _returnvalue_3)
      (else
        (Actor|DestroyActor _returnvalue_3 :!pinned true) ; If couldnt attach link to start concept\ndestroy link
        (return false 0)))
    (else
      (return false 0))))

(fn LoadAnnotation
  (params (AnnotationData :type S%20Concept%20Annotation%20Structure))
  (bind _conceptactors (Variables|Default|GetConceptActors))
  (bind _concept_id (Utilities|Struct|BreakS_ConceptAnnotation AnnotationData))
  (bind (_value _returnvalue) (Utilities|Map|Find _conceptactors _concept_id))
  (if _returnvalue ; Find concept actor related\nto the annotation
    (Default|AddAnnotation _value AnnotationData)
    (return true)
    (else
      (return false))))

(fn ConfigureParameters
  (params (HideConcepts :type Boolean) (HideLinks :type Boolean) (UseSecondaryBox :type Boolean) (UseTertiaryBox :type Boolean))
  (Utilities|FlowControl|Sequence
    (:then_0
      (Variables|Default|SetHideConcepts HideConcepts))
    (:then_1
      (Variables|Default|SetHideLinks HideLinks))
    (:then_2
      (Variables|Default|SetUseSecondaryBox UseSecondaryBox))
    (:then_3
      (Variables|Default|SetUseTertiaryBox UseTertiaryBox))))

(fn RepositionConcepts
  (bind _returnvalue (Class|KismetSystemLibrary|MakeLiteralInteger 4))
  (bind _tertiarybox (Variables|Default|GetTertiaryBox))
  (bind (_origin _boxextent) (Collision|GetComponentBounds _tertiarybox))
  (bind _returnvalue_2 (* _returnvalue 2))
  (bind _returnvalue_3 (- _returnvalue_2 2))
  (bind _returnvalue_4 (- (.z _origin) (.z _boxextent)))
  (Utilities|FlowControl|Sequence
    (:then_0
      ;[0 0 0] BubbleSort concept in order of first mention
      (bind _values (Utilities|Map|Values (Variables|Default|GetConceptActors)))
      (bind _output_get (LocalVariables|SetLocal_SortedConcepts _values))
      (for _index (range 0 (Utilities|Array|LastIndex _output_get))
        (for _index_2 (range _index (Utilities|Array|LastIndex _output_get))
          (bind _timespan (Default|GetEarliestMention (Utilities|Array|Get(acopy) _output_get _index_2)))
          (bind _timespan_2 (Default|GetEarliestMention (Utilities|Array|Get(acopy) _output_get _index)))
          (if (> _timespan_2 _timespan)
            (Utilities|Array|Swap _output_get _index_2 _index)))))
    (:then_1
      ;[0 0 0] Find most mentioned concept time
      (for _array_element (LocalVariables|GetLocal_SortedConcepts)
        (bind _totalseconds (Default|GetTotalMention _array_element))
        (if (> _totalseconds (LocalVariables|GetLocal_BiggestConcept))
          (LocalVariables|SetLocal_BiggestConcept _totalseconds))))
    (:then_2
      ;[0 0 0] Reposition concept on XYZ coordinates
      (for (_array_element_2 _array_index) (LocalVariables|GetLocal_SortedConcepts)
        (bind _totalseconds_2 (Default|GetTotalMention _array_element_2))
        (Transformation|SetActorLocation _array_element_2 (Math|Vector|MakeVector (- (+ (.x _origin) (.x _boxextent)) (* _array_index (/ (* (.x _boxextent) 2.0) (Utilities|Array|Length (LocalVariables|GetLocal_SortedConcepts))))) (+ (- (.y _origin) (.y _boxextent)) (* (* (.y _boxextent) 2.0) (Math|Float|SafeDivide (* (Math|Float|Absolute(Float) (- (Math|Integer|%(Integer) _array_index (- _returnvalue_2 2)) (/ _returnvalue_3 2.0))) 2.0) _returnvalue_3))) (Math|Float|Lerp _returnvalue_4 (+ _returnvalue_4 (* (.z _boxextent) 2.0)) (Math|Float|SafeDivide _totalseconds_2 (LocalVariables|GetLocal_BiggestConcept)))) false true)))))

(fn SpawnConceptB
  (params (ConceptData :type S%20Concept%20Structure))
  (bind _primarybox (Variables|Default|GetPrimaryBox))
  (bind _usesecondarybox (Variables|Default|GetUseSecondaryBox))
  (bind _secondarybox (Variables|Default|GetSecondaryBox))
  (bind _returnvalue (select _usesecondarybox _secondarybox _primarybox))
  (bind (_origin _boxextent) (Collision|GetComponentBounds _returnvalue))
  (bind _returnvalue_2 (Game|SpawnActorfromClass "/Game/Blueprints/BP_Concept.BP_Concept_C" (Math|Transform|MakeTransform (Math|Random|RandomPointinBoundingBox _origin _boxextent) "0, 0, 0" (Math|Conversions|ToVector(Float) (Variables|Default|GetConceptScale))) "AdjustIfPossibleButAlwaysSpawn" "MultiplyWithRoot" 0 0 :!pinned true)) ; Spawn concept actor
  ;[1 1 1] Initialise concept actor with data
  (Default|SetConceptData _returnvalue_2 ConceptData)
  (Default|SetAnnotationMenu _returnvalue_2 (Variables|Default|GetAnnotationMenu))
  (Default|SetVisibility _returnvalue_2 (not (Variables|Default|GetHideConcepts)))
  (return true _returnvalue_2))

(fn RepositionConceptsB
  (bind _returnvalue (Class|KismetSystemLibrary|MakeLiteralInteger 4))
  (bind _primarybox (Variables|Default|GetPrimaryBox))
  (bind (_origin _boxextent) (Collision|GetComponentBounds _primarybox))
  (bind _returnvalue_2 (* _returnvalue 2))
  (bind _returnvalue_3 (- _returnvalue_2 2))
  (bind _returnvalue_4 (- (.z _origin) (.z _boxextent)))
  (Utilities|FlowControl|Sequence
    (:then_0
      ;[0 0 0] BubbleSort concept in order of first mention
      (bind _values (Utilities|Map|Values (Variables|Default|GetConceptActors)))
      (bind _output_get (LocalVariables|SetLocal_SortedConcepts _values))
      (for _index (range 0 (Utilities|Array|LastIndex _output_get))
        (for _index_2 (range _index (Utilities|Array|LastIndex _output_get))
          (bind _timespan (Default|GetEarliestMention (Utilities|Array|Get(acopy) _output_get _index_2)))
          (bind _timespan_2 (Default|GetEarliestMention (Utilities|Array|Get(acopy) _output_get _index)))
          (if (> _timespan_2 _timespan)
            (Utilities|Array|Swap _output_get _index_2 _index)))))
    (:then_1
      ;[0 0 0] Find most mentioned concept time
      (for _array_element (LocalVariables|GetLocal_SortedConcepts)
        (bind _totalseconds (Default|GetTotalMention _array_element))
        (if (> _totalseconds (LocalVariables|GetLocal_BiggestConcept))
          (LocalVariables|SetLocal_BiggestConcept _totalseconds))))
    (:then_2
      ;[0 0 0] Reposition concept on XYZ coordinates
      (for (_array_element_2 _array_index) (LocalVariables|GetLocal_SortedConcepts)
        (bind _totalseconds_2 (Default|GetTotalMention _array_element_2))
        (Transformation|SetActorLocation _array_element_2 (Math|Vector|MakeVector (- (+ (.x _origin) (.x _boxextent)) (* _array_index (/ (* (.x _boxextent) 2.0) (Utilities|Array|Length (LocalVariables|GetLocal_SortedConcepts))))) (+ (- (.y _origin) (.y _boxextent)) (* (* (.y _boxextent) 2.0) (Math|Float|SafeDivide (* (Math|Float|Absolute(Float) (- (Math|Integer|%(Integer) _array_index (- _returnvalue_2 2)) (/ _returnvalue_3 2.0))) 2.0) _returnvalue_3))) (Math|Float|Lerp _returnvalue_4 (+ _returnvalue_4 (* (.z _boxextent) 2.0)) (Math|Float|SafeDivide _totalseconds_2 (LocalVariables|GetLocal_BiggestConcept)))) false true)))))

(fn NewFunction)