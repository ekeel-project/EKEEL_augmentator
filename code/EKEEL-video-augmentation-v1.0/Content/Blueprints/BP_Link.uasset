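; Link actor that draws a Niagara effect toward an end actor and shows the link data's label in a widget.
; A looping timer keeps the label's scene component at the midpoint between the link and end actor.
; Another toggleable timer rotates it toward a given component.
; Visibility follows the attach parent's and end actor's hidden states plus a BeenMentioned flag, and the link supports colour changes and timed deletion.
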(event Custom|PositionLabel
  ;[1 1 1] Events used for initialisation
  (Utilities|IsValid (Variables|Default|GetEndActor)
    (:Is%20Valid
      (bind _midpoint (CallFunction|FindMidpointData self (Variables|Default|GetEndActor)))
      (Transformation|SetWorldLocation (Variables|Default|GetScene) _midpoint false true))))

(event Custom|RotateLabel
  ;[1 1 1] Events related to the label widget holding the text value representing the
  ; link name, such as the rotation of it towards a specified SceneComponent,
  ; these events should be used whenever an actor is in range of the link name.
  (bind _labelrotationtarget (Variables|Default|GetLabelRotationTarget)
    (:then
      (Transformation|SetWorldRotation (Variables|Default|GetScene) (Math|Rotator|FindLookatRotation (Transformation|GetWorldLocation (Variables|Default|GetScene)) (Transformation|GetWorldLocation _labelrotationtarget)) false false))
    (:else)))

(event Custom|ActivateDeletion
  (params (Time :type Float%20%28single-precision%29))
  ;[1 1 1] Events related to the link removal, immediate and after a specified
  ; amount of time in seconds have passed.
  (Actor|SetLifeSpan Time))

(event Custom|DeleteLink
  ;[1 1 1] Events related to the link removal, immediate and after a specified
  ; amount of time in seconds have passed.
  (Actor|DestroyActor))

(event Custom|EnableLabelRotation
  (params (FacingComponent :type Scene%20Component%20Object%20Reference))
  ;[1 1 1] Events related to the label widget holding the text value representing the
  ; link name, such as the rotation of it towards a specified SceneComponent,
  ; these events should be used whenever an actor is in range of the link name.
  (Utilities|IsValid FacingComponent
    (:Is%20Valid
      (Variables|Default|SetLabelRotationTarget FacingComponent)
      (bind _returnvalue (Utilities|Time|SetTimerbyFunctionName 0 "RotateLabel" 0.02 true :!pinned true)) ; Start rotating label towards a scene component
    )))

(event Custom|DisableLabelRotation
  ;[1 1 1] Events related to the label widget holding the text value representing the
  ; link name, such as the rotation of it towards a specified SceneComponent,
  ; these events should be used whenever an actor is in range of the link name.
  (Utilities|Time|ClearandInvalidateTimerbyHandle (stale Custom|EnableLabelRotation _returnvalue)))

(event EventBeginPlay
  ;[1 1 1] Events used for initialisation
  (Utilities|Time|SetTimerbyFunctionName 0 "PositionLabel" 0.01 true :!pinned true) ; Start updating label on midpoint
  (CallFunction|SetLinkData (Variables|Default|GetLinkData) :!pinned true) ; Set link data on begin play,\nthis will update the widget label
)

(fn ConstructionScript
  (CallFunction|SetLinkData (Variables|Default|GetLinkData))
  (CallFunction|SetEndActor (Variables|Default|GetEndActor))
  (CallFunction|UpdateVisibility)
  (CallFunction|PositionLabel))

(fn SetLinkData
  (params (LinkData :type S%20Link%20Structure))
  (bind _output_get (Variables|Default|SetLinkData LinkData))
  (CallFunction|SetLabel (Utilities|Text|ToText(String) (.label (Utilities|Struct|BreakS_Link _output_get)))) ; Update the link label
)

(fn GetLinkData
  (return (Variables|Default|GetLinkData)) ; Returns the information of the link
)

(fn SetEndActor
  (params (EndActor :type Actor%20Object%20Reference))
  (bind _output_get (Variables|Default|SetEndActor EndActor))
  (Class|NiagaraComponent|SetVariableObject (Variables|Default|GetNiagaraComponent) "User.ActorEnd" _output_get) ; Update niagara system end point
)

(fn GetEndActor
  (return (Variables|Default|GetEndActor)) ; Retrieves the end point actor
)

(fn SetLinkColour
  (params (Colour :type Linear%20Color%20Structure))
  (Effects|Components|ParticleSystem|SetColorParameter (Variables|Default|GetNiagaraComponent) "User.Colour" Colour) ; Update niagara system colour
)

(fn SetLabelVisibility
  (params (NewVisibility :type Boolean))
  (Rendering|SetVisibility (Variables|Default|GetWidgetLabel) NewVisibility false))

(fn UpdateVisibility
  (bind _returnvalue (Actor|GetAttachParentActor))
  (bind _bhidden (Variables|Rendering|GetbHidden))
  (bind _endactor (Variables|Default|GetEndActor))
  (bind _beenmentioned (Variables|Default|GetbeenMentioned))
  (bind _bhidden_2 (Variables|Rendering|GetbHidden))
  (bind _returnvalue_2 (Class|KismetMathLibrary|XORBoolean _beenmentioned _bhidden))
  (bind _returnvalue_3 (and _returnvalue_2 _bhidden_2))
  (if (!= (Variables|Rendering|GetbHidden) _returnvalue_3) ; Update only if the final value\nwill be different
    (if (and (Utilities|IsValid _returnvalue) (Utilities|IsValid _endactor)) ; Update only if both end points\nare valid
      (if (or (Variables|/Script/Engine.Actor|GetbHidden _returnvalue) (Variables|/Script/Engine.Actor|GetbHidden _endactor)) ; Check if either end point is\nhidden
        (Rendering|SetActorHiddenInGame true) ; Link hidden if either end point is hidden
        (else
          (Rendering|SetActorHiddenInGame _returnvalue_3))))))

(fn SetLabel
  (params (Text :type Text))
  (bind _aswbp_label (Utilities|Casting|CastToWBP_Label (UserInterface|GetWidget (Variables|Default|GetWidgetLabel))))
  (Default|SetLabel _aswbp_label Text))

(fn SetVisibility
  (params (NewVisibility :type Boolean))
  (Rendering|SetActorHiddenInGame (not NewVisibility)))

(fn FindMidpointData
  (params (ActorOne :type Actor%20Object%20Reference) (ActorTwo :type Actor%20Object%20Reference))
  (bind _returnvalue (Transformation|GetActorLocation ActorOne))
  (bind _returnvalue_2 (Transformation|GetActorLocation ActorTwo))
  (return (+ (/ (- _returnvalue _returnvalue_2) 2) _returnvalue_2) (Math|Rotator|FindLookatRotation _returnvalue _returnvalue_2)))