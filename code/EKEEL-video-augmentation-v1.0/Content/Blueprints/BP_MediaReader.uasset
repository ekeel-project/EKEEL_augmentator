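; Media reader module actor that turns video data from a linked JsonReader into a map of FileMediaSource objects keyed by video ID.
; On the JsonReader's ReadComplete, it builds each file path from the ID, prefix and path type (full, project or content directory), adding a default extension if none is present.
; Only existing files are added, with optional Logger reporting.
; MediaMapCreated fires a tick after the loop to notify other modules.
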(event Custom|ReadVideoFiles
  (bind _logger (Variables|Default|GetLogger))
  (bind _logger_2 (Variables|Default|GetLogger))
  (bind _logger_3 (Variables|Default|GetLogger))
  ;[1 1 1] FUNCTIONALITY
  ; Events related to the functionality of the module, executing the primary functions
  ; when required, typically bound to other modules to react and execute when data
  ; has been correctly instanced.
  (Variables|Default|GetJsonReader
    (:then
      (Utilities|FlowControl|Sequence
        (:then_0
          (bind _videos (Default|GetVideos (Variables|Default|GetJsonReader) :!pinned true)) ; Retrieve video data from JsonReader
          (for _array_element _videos ; Loop for every video structure created by the JsonReader\nand try constructing the FileMediaSource object to insert\nin the MediaMap
            (bind (_valid _filemediasource) (CallFunction|ConstructMedia _array_element))
            (if _valid
              (Utilities|Map|Add (Variables|Default|GetMediaMap) (Utilities|Struct|BreakS_Video _array_element) _filemediasource :!pinned true) ; Add media object if file exists
              ;;[0.1677 1 0] Log: FileMediaSource successfully created
              (Utilities|IsValid _logger_3
                (:Is%20Valid
                  (Default|Log _logger_3 "MediaReader" "Log" (Utilities|String|Append "FileMediaSource | added ID: " (Utilities|Struct|BreakS_Video _array_element)) (Variables|Default|GetLog))))
              (else
                (Utilities|FlowControl|Sequence
                  (:then_0
                    ;;[1 0.9098 0] Warning: Could not create FileMediaSource
                    (Utilities|IsValid _logger_2
                      (:Is%20Valid
                        (Default|Log _logger_2 "MediaReader" "Warning" "FileMediaSource | Could not create object" (Variables|Default|GetLog)))))
                  (:then_1
                    (Development|PrintString "Could not read media file into an object")))))))
        (:then_1
          (Utilities|FlowControl|Sequence :!pinned true ; Dispatch MediaMapCreated
            (:then_0
              ;;[0.1677 1 0] Log: Completed creating MediaMap
              (Utilities|IsValid _logger
                (:Is%20Valid
                  (Default|Log _logger "MediaReader" "Log" "Completed creating MediaMap, calling MediaMapCreated" (Variables|Default|GetLog)))))
            (:then_1
              (Utilities|FlowControl|DelayUntilNextTick)
              (Default|CallMediaMapCreated))))))
    (:else)))

(event EventBeginPlay
  ;[1 1 1] INITIALISATION
  ; Initialisation events that set up the module variables and bind events to other
  ; connected modules if present.
  (Utilities|FlowControl|Sequence
    (:then_0
      (if (and (not (Utilities|IsValid (Variables|Default|GetLogger))) (Variables|Default|GetLog))
        (Development|PrintString "[Warning][MediaReader] Logging enabled but no Logger specified.")))
    (:then_1
      (bind _jsonreader (Variables|Default|GetJsonReader :!pinned true) ; Bind ReadVideoFiles to JsonReader\nReadComplete dispatcher
        (:then
          (EventDispatchers|BindEventtoReadComplete _jsonreader (delegate Custom|ReadVideoFiles)))
        (:else
          (Development|PrintString "[Warning][MediaReader] JsonReader not specified."))))))

(fn ConstructionScript)

(fn GetMediaMap
  (return (Variables|Default|GetMediaMap)) ; Returns the array of successfully created\nFileMediaSource objects
)

(fn ConstructMedia
  (params (VideoData :type S%20Video%20Structure))
  (bind _filepath (CallFunction|ConstructPath (Variables|Default|GetPathType) (Variables|Default|GetPathPrefix) (Utilities|Struct|BreakS_Video VideoData) :!pinned true)) ; Construct path
  (if (Class|BlueprintPathsLibrary|FileExists (select (Utilities|Array|IsEmpty (Class|BlueprintPathsLibrary|GetExtension _filepath false)) (Utilities|String|Append _filepath (Variables|Default|GetDefaultFileExtension)) _filepath)) ; Verify if file exists
    (bind _returnvalue (Game|ConstructObjectfromClass "/Script/MediaAssets.FileMediaSource"))
    (Class|FileMediaSource|SetFilePath _returnvalue (select (Utilities|Array|IsEmpty (Class|BlueprintPathsLibrary|GetExtension _filepath false)) (Utilities|String|Append _filepath (Variables|Default|GetDefaultFileExtension)) _filepath)) ; Set the file path to the constructed\nFileMediaSource object
    (return true _returnvalue)
    (else
      (return false 0))))

(fn ConstructPath
  (params (PathType :type PathType%20Enum :default "NewEnumerator0") (Prefix :type String) (FileName :type String))
  (switch Utilities|FlowControl|Switch|SwitchonPathType PathType
    (:NewEnumerator0
      (return (Utilities|String|Append (Utilities|String|MakeLiteralString Prefix) FileName)))
    (:NewEnumerator1
      (return (Utilities|String|Append (Utilities|String|MakeLiteralString (Class|KismetSystemLibrary|GetProjectDirectory)) Prefix FileName)))
    (:NewEnumerator2
      (return (Utilities|String|Append (Utilities|String|MakeLiteralString (Class|KismetSystemLibrary|GetProjectContentDirectory)) Prefix FileName)))))