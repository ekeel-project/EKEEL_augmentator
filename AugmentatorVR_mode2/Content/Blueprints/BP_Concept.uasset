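; Actor representing a concept node, with a label widget, timestamped annotations shown through an annotation menu actor, and lookup of attached BP_Link actors to other concepts.
; A hidden concept that is mentioned gets revealed with collision and a timeline move from its initial position.
; Focused, mentioned and previously mentioned states set custom depth stencil values for highlighting.
; An optional looping timer turns the label toward a target component.
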(event Custom|TransitionFromTo
  (params (FromWorldPosition :type Vector) (ToWorldPosition :type Vector))
  ;[1 1 1] Events used for initialisation
  (bind _alpha (Timeline|Timeline Play)
    (:Update
      (Transformation|SetActorLocation (Math|Vector|Lerp(Vector) FromWorldPosition ToWorldPosition _alpha) false true))))

(event Custom|RotateLabel
  ;[1 1 1] Events related to the rotation of the widget component which visualises the concept
  ; name in order for it to always face a certain scene component.
  (bind _labelrotationtarget (Variables|Default|GetLabelRotationTarget)
    (:then
      (Transformation|SetWorldRotation (Variables|Default|GetScene) (Math|Rotator|FindLookatRotation (Transformation|GetWorldLocation (Variables|Default|GetScene)) (Transformation|GetWorldLocation _labelrotationtarget)) false false))
    (:else)))

(event Custom|EnableLabelRotation
  (params (FacingComponent :type Scene%20Component%20Object%20Reference))
  ;[1 1 1] Events related to the rotation of the widget component which visualises the concept
  ; name in order for it to always face a certain scene component.
  (Utilities|IsValid FacingComponent
    (:Is%20Valid
      (Variables|Default|SetLabelRotationTarget FacingComponent)
      (bind _returnvalue (Utilities|Time|SetTimerbyFunctionName 0 "RotateLabel" 0.02 true :!pinned true)) ; Start rotating label towards a scene component
    )))

(event Custom|DisableLabelRotation
  ;[1 1 1] Events related to the rotation of the widget component which visualises the concept
  ; name in order for it to always face a certain scene component.
  (Utilities|Time|ClearandInvalidateTimerbyHandle (stale Custom|EnableLabelRotation _returnvalue)))

(event EventBeginPlay
  ;[1 1 1] Events used for initialisation
  (CallFunction|SetConceptData (Variables|Default|GetConceptData) :!pinned true) ; Set concept data on begin play,\nthis will update the widget label
)

(fn ConstructionScript
  (CallFunction|SetConceptData (Variables|Default|GetConceptData))
  (CallFunction|UpdateVisibility)
  (CallFunction|UpdateHighlight)
  (Variables|Default|SetInitialPosition (Transformation|GetActorLocation)))

(fn SetConceptData
  (params (ConceptData :type S%20Concept%20Structure))
  (bind _output_get (Variables|Default|SetConceptData ConceptData))
  (CallFunction|SetLabel (Utilities|Text|ToText(String) (.label (Utilities|Struct|BreakS_Concept _output_get)))) ; Update the link label
)

(fn GetConceptData
  (return (Variables|Default|GetConceptData)) ; Returns the information of the concept
)

(fn SetAnnotationsData
  (params (AnnotationsData :type Array%20of%20S%20Concept%20Annotation%20Structures))
  (Variables|Default|SetConceptAnnotations AnnotationsData))

(fn GetAnnotationsData
  (return (Variables|Default|GetConceptAnnotations)) ; Returns the information of the annotations\nrelated to this concept
)

(fn SetAnnotationMenu
  (params (AnnotationMenu :type BP%20Annotation%20Menu%20Object%20Reference))
  (Variables|Default|SetAnnotationMenu AnnotationMenu))

(fn GetAnnotationMenu
  (return (Variables|Default|GetAnnotationMenu)) ; Retrieves the actor where the annotations\nwill be visualised when opened
)

(fn SetLabel
  (params (Text :type Text))
  (bind _aswbp_label (Utilities|Casting|CastToWBP_Label (UserInterface|GetWidget (Variables|Default|GetWidgetLabel))))
  (Default|SetLabel _aswbp_label Text))

(fn SetVisibility
  (params (NewVisibility :type Boolean))
  (Rendering|SetActorHiddenInGame (not NewVisibility))
  (Collision|SetActorEnableCollision NewVisibility) ; Remove collisions if not visible
)

(fn UpdateVisibility
  (bind _ismentioned (Variables|Default|GetisMentioned))
  (bind _bhidden (Variables|Rendering|GetbHidden))
  (bind _bhidden_2 (Variables|Rendering|GetbHidden))
  (bind _returnvalue (Class|KismetMathLibrary|XORBoolean _ismentioned _bhidden))
  (bind _returnvalue_2 (and _returnvalue _bhidden_2))
  (if (!= (Variables|Rendering|GetbHidden) _returnvalue_2) ; Update only if the final value\nwill be different
    (CallFunction|Transitionfromto (Variables|Default|GetInitialPosition) (Transformation|GetActorLocation)) ; Start animating the position from the \ninitial position to the current position
    (Rendering|SetActorHiddenInGame _returnvalue_2)
    (Collision|SetActorEnableCollision (not _returnvalue_2))))

(fn UpdateHighlight
  (if (Variables|Default|GetisFocused)
    (Rendering|SetCustomDepthStencilValue (Variables|Default|GetStaticMesh) 1)
    (elif (Variables|Default|GetisMentioned)
      (Rendering|SetCustomDepthStencilValue (Variables|Default|GetStaticMesh) 2)
      (elif (Variables|Default|GetbeenMentioned)
        (Rendering|SetCustomDepthStencilValue (Variables|Default|GetStaticMesh) 3)
        (else
          (Rendering|SetCustomDepthStencilValue (Variables|Default|GetStaticMesh) 0))))))

(fn OpenMenu
  (bind _annotationmenu (Variables|Default|GetAnnotationMenu)
    (:then
      (Default|OpenMenu _annotationmenu (Variables|Default|GetConceptData) (Variables|Default|GetConceptAnnotations)))
    (:else)))

(fn AddAnnotation
  (params (AnnotationData :type S%20Concept%20Annotation%20Structure))
  (Utilities|Array|AddUnique (Variables|Default|GetConceptAnnotations) AnnotationData))

(fn CheckLink
  (params (EndConcept :type BP%20Concept%20Object%20Reference))
  (for _array_element (Actor|GetAttachedActors false false) ; Scan the actors attached to the concept
    (bind _asbp_link (Utilities|Casting|CastToBP_Link _array_element))
    (bind _endactor (Default|GetEndActor _asbp_link))
    (if (== _endactor EndConcept) ; Check if link from the concept\nconnects the given concept
      (return true _asbp_link)))
  (return false 0))

(fn GetEarliestMention
  (bind _conceptannotations (Variables|Default|GetConceptAnnotations))
  (if (Utilities|Array|IsNotEmpty (Variables|Default|GetConceptAnnotations))
    (LocalVariables|SetEarliestTimespan (.start_timestamp (Utilities|Struct|BreakS_ConceptAnnotation (Utilities|Array|Get(acopy) _conceptannotations))))
    (for _array_element _conceptannotations
      (if (< (.start_timestamp (Utilities|Struct|BreakS_ConceptAnnotation _array_element)) (LocalVariables|GetEarliestTimespan))
        (LocalVariables|SetEarliestTimespan (.start_timestamp (Utilities|Struct|BreakS_ConceptAnnotation _array_element)))))
    (return (LocalVariables|GetEarliestTimespan))
    (else
      (return (Math|Timespan|MakeTimespan 9999 0 0 0 0)))))

(fn GetTotalMention
  (for _array_element (Variables|Default|GetConceptAnnotations)
    (LocalVariables|SetTotalMention (+ (LocalVariables|GetTotalMention) (Math|Timespan|GetTotalSeconds (- (.end_timestamp (Utilities|Struct|BreakS_ConceptAnnotation _array_element)) (.start_timestamp (Utilities|Struct|BreakS_ConceptAnnotation _array_element)))))))
  (return (LocalVariables|GetTotalMention)))