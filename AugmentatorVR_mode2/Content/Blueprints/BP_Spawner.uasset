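; Spawner module that builds concept and link actors from JsonReader data once ReadComplete fires.
; Concepts spawn randomly in the primary or secondary box, links attach between their endpoint concepts, and annotations are added to concepts.
; It then repositions concepts within PrimaryBox: sorted by earliest mention along X, triangle-waved on Y, raised on Z by total mention.
; Results are optionally logged, and SpawnComplete fires a tick later.
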(event Custom|Spawn
  (bind _logger (Variables|Default|GetLogger))
  (bind _logger_2 (Variables|Default|GetLogger))
  (bind _logger_3 (Variables|Default|GetLogger))
  (bind _logger_4 (Variables|Default|GetLogger))
  (bind _logger_5 (Variables|Default|GetLogger))
  (bind _logger_6 (Variables|Default|GetLogger))
  (bind _logger_7 (Variables|Default|GetLogger))
  ;[1 1 1] Events related to the primary function of the Spawner module which will
  ; generate the concepts, links and annotations using the parameters of
  ; the spawner and log the results if logging is enabled.
  (Utilities|FlowControl|Sequence
    (:then_0
      (if (Variables|Default|GetSpawnConcepts)
        (bind _jsonreader (Variables|Default|GetJsonReader)
          (:then
            (bind _concepts (Default|GetConcepts _jsonreader))
            (for _array_element _concepts ; Try spawning all concepts
              (bind (_valid _concept) (CallFunction|SpawnConcept _array_element))
              (if _valid
                (Utilities|Map|Add (Variables|Default|GetConceptActors) (.id (Utilities|Struct|BreakS_Concept _array_element)) _concept)
                ;;[0.1677 1 0] Log: Concept actor successfully spawned
                (Utilities|IsValid _logger
                  (:Is%20Valid
                    (Default|Log _logger "Spawner" "Log" (Utilities|String|Append "Concept | added ID: " (.id (Utilities|Struct|BreakS_Concept _array_element))) (Variables|Default|GetLog))))
                (else
                  ;;[1 0.9098 0] Warning: Could not spawn concept actor
                  (Utilities|IsValid _logger_2
                    (:Is%20Valid
                      (Default|Log _logger_2 "Spawner" "Warning" "Concept | Could not spawn actor" (Variables|Default|GetLog))))))))
          (:else))))
    (:then_1
      (if (Variables|Default|GetSpawnLinks)
        (bind _jsonreader_2 (Variables|Default|GetJsonReader)
          (:then
            (bind _links (Default|GetLinks _jsonreader_2))
            (for _array_element_2 _links ; Try spawning all links
              (bind (_valid_2 _link) (CallFunction|SpawnLink _array_element_2))
              (if _valid_2
                (Utilities|Map|Add (Variables|Default|GetLinkActors) (.link_id (Utilities|Struct|BreakS_Link _array_element_2)) _link)
                ;;[0.1677 1 0] Log: Link actor successfully spawned
                (Utilities|IsValid _logger_3
                  (:Is%20Valid
                    (Default|Log _logger_3 "Spawner" "Log" (Utilities|String|Append "Link | added ID: " (.link_id (Utilities|Struct|BreakS_Link _array_element_2))) (Variables|Default|GetLog))))
                (else
                  ;;[1 0.9098 0] Warning: Could not spawn link actor
                  (Utilities|IsValid _logger_4
                    (:Is%20Valid
                      (Default|Log _logger_4 "Spawner" "Warning" "Link | Could not spawn actor" (Variables|Default|GetLog))))))))
          (:else))))
    (:then_2
      (if (Variables|Default|GetLoadAnnotations)
        (bind _jsonreader_3 (Variables|Default|GetJsonReader)
          (:then
            (bind _annotations (Default|GetAnnotations _jsonreader_3))
            (for _array_element_3 _annotations ; Try adding all annotations
              (bind _valid_3 (CallFunction|LoadAnnotation _array_element_3))
              (if _valid_3
                ;;[0.1677 1 0] Log: Annotation successfully added
                (Utilities|IsValid _logger_7
                  (:Is%20Valid
                    (Default|Log _logger_7 "Spawner" "Log" (Utilities|String|Append "Annotation | added ID: " (.ann_id (Utilities|Struct|BreakS_ConceptAnnotation _array_element_3))) (Variables|Default|GetLog))))
                (else
                  ;;[1 0.9098 0] Warning: Could not add annotation
                  (Utilities|IsValid _logger_6
                    (:Is%20Valid
                      (Default|Log _logger_6 "Spawner" "Warning" "Annotation | Could not add annotation" (Variables|Default|GetLog))))))))
          (:else))))
    (:then_3
      (CallFunction|RepositionConcepts :!pinned true) ; Reposition Concepts
    )
    (:then_4
      (Utilities|FlowControl|Sequence :!pinned true ; Dispatch SpawnComplete
        (:then_0
          ;;[0.1677 1 0] Log: Completed spawning operation
          (Utilities|IsValid _logger_5
            (:Is%20Valid
              (Default|Log _logger_5 "Spawner" "Log" "Completed spawning actors, calling SpawnComplete" (Variables|Default|GetLog)))))
        (:then_1
          (Utilities|FlowControl|DelayUntilNextTick)
          (Default|CallSpawnComplete))))))

(event EventBeginPlay
  ;[1 1 1] Events used for initialisation purposes of the module and binding to other modules
  ; to request data when it has been successfully created.
  (Utilities|FlowControl|Sequence
    (:then_0
      (if (and (not (Utilities|IsValid (Variables|Default|GetLogger))) (Variables|Default|GetLog))
        (Development|PrintString "[Warning][Spawner] Logging enabled but no Logger specified.")))
    (:then_1
      (Variables|Default|GetAnnotationMenu
        (:then)
        (:else
          (Development|PrintString "[Warning][Spawner] AnnotationMenu not specified."))))
    (:then_2
      (bind _jsonreader (Variables|Default|GetJsonReader :!pinned true) ; Bind Spawn to JsonReader\nReadComplete dispatcher
        (:then
          (EventDispatchers|BindEventtoReadComplete _jsonreader (delegate Custom|Spawn)))
        (:else
          (Development|PrintString "[Warning][Spawner] JsonReader not specified."))))))

(fn ConstructionScript)

(fn GetConceptActorMap
  (return (Variables|Default|GetConceptActors)) ; Returns the generated concept actors
)

(fn GetLinkActorMap
  (return (Variables|Default|GetLinkActors)) ; Returns the generated link actors
)

(fn SpawnConcept
  (params (ConceptData :type S%20Concept%20Structure))
  (bind _usesecondarybox (Variables|Default|GetUseSecondaryBox))
  (bind _secondarybox (Variables|Default|GetSecondaryBox))
  (bind _primarybox (Variables|Default|GetPrimaryBox))
  (bind _returnvalue (select _usesecondarybox _secondarybox _primarybox))
  (bind (_origin _boxextent) (Collision|GetComponentBounds _returnvalue))
  (bind _returnvalue_2 (Game|SpawnActorfromClass "/Game/Blueprints/BP_Concept.BP_Concept_C" (Math|Transform|MakeTransform (Math|Random|RandomPointinBoundingBox _origin _boxextent) "0, 0, 0" (Math|Conversions|ToVector(Float) (Variables|Default|GetConceptScale))) "AdjustIfPossibleButAlwaysSpawn" "MultiplyWithRoot" 0 0 :!pinned true)) ; Spawn concept actor
  ;[1 1 1] Initialise concept actor with data
  (Default|SetConceptData _returnvalue_2 ConceptData)
  (Default|SetAnnotationMenu _returnvalue_2 (Variables|Default|GetAnnotationMenu))
  (Default|SetVisibility _returnvalue_2 (not (Variables|Default|GetHideConcepts)))
  (return true _returnvalue_2))

(fn SpawnLink
  (params (LinkData :type S%20Link%20Structure))
  (bind _conceptactors (Variables|Default|GetConceptActors))
  (bind (_start_concept_id _end_concept_id) (Utilities|Struct|BreakS_Link LinkData))
  (bind (_value _returnvalue) (Utilities|Map|Find _conceptactors _start_concept_id))
  (bind (_value_2 _returnvalue_2) (Utilities|Map|Find _conceptactors _end_concept_id))
  (if (and _returnvalue _returnvalue_2) ; If concept end points are\nmissing avoid spawning
    (bind _returnvalue_3 (Game|SpawnActorfromClass "/Game/Blueprints/BP_Link.BP_Link_C" (Math|Transform|MakeTransform "0, 0, 0" "0, 0, 0" (Math|Conversions|ToVector(Float) (Variables|Default|GetLinkScale))) "Undefined" "MultiplyWithRoot" 0 0 :!pinned true)) ; Spawn link actor
    ;[1 1 1] Initialise link actor with data
    (Default|SetLinkData _returnvalue_3 LinkData)
    (Default|SetLinkColour _returnvalue_3 (Variables|Default|GetLinkColour))
    (Default|SetLabelVisibility _returnvalue_3 (Variables|Default|GetLinkLabels))
    (Default|SetVisibility _returnvalue_3 (not (Variables|Default|GetHideLinks)))
    (Default|SetEndActor _returnvalue_3 _value_2) ; Set end point
    (bind _returnvalue_4 (Transformation|AttachActorToActor _returnvalue_3 _value "None" "KeepRelative" "KeepWorld" "KeepWorld" false)) ; Set start point by attaching to another actor
    (if _returnvalue_4
      (return true _returnvalue_3)
      (else
        (Actor|DestroyActor _returnvalue_3 :!pinned true) ; If couldnt attach link to start concept\ndestroy link
        (return false 0)))
    (else
      (return false 0))))

(fn LoadAnnotation
  (params (AnnotationData :type S%20Concept%20Annotation%20Structure))
  (bind _conceptactors (Variables|Default|GetConceptActors))
  (bind _concept_id (Utilities|Struct|BreakS_ConceptAnnotation AnnotationData))
  (bind (_value _returnvalue) (Utilities|Map|Find _conceptactors _concept_id))
  (if _returnvalue ; Find concept actor related\nto the annotation
    (Default|AddAnnotation _value AnnotationData)
    (return true)
    (else
      (return false))))

(fn ConfigureParameters
  (params (HideConcepts :type Boolean) (HideLinks :type Boolean) (UseSecondaryBox :type Boolean))
  (Utilities|FlowControl|Sequence
    (:then_0
      (Variables|Default|SetHideConcepts HideConcepts))
    (:then_1
      (Variables|Default|SetHideLinks HideLinks))
    (:then_2
      (Variables|Default|SetUseSecondaryBox UseSecondaryBox))))

(fn RepositionConcepts
  (bind _returnvalue (Class|KismetSystemLibrary|MakeLiteralInteger 4))
  (bind _primarybox (Variables|Default|GetPrimaryBox))
  (bind (_origin _boxextent) (Collision|GetComponentBounds _primarybox))
  (bind _returnvalue_2 (* _returnvalue 2))
  (bind _returnvalue_3 (- _returnvalue_2 2))
  (bind _returnvalue_4 (- (.z _origin) (.z _boxextent)))
  (Utilities|FlowControl|Sequence
    (:then_0
      ;[0 0 0] BubbleSort concept in order of first mention
      (bind _values (Utilities|Map|Values (Variables|Default|GetConceptActors)))
      (bind _output_get (LocalVariables|SetLocal_SortedConcepts _values))
      (for _index (range 0 (Utilities|Array|LastIndex _output_get))
        (for _index_2 (range _index (Utilities|Array|LastIndex _output_get))
          (bind _timespan (Default|GetEarliestMention (Utilities|Array|Get(acopy) _output_get _index_2)))
          (bind _timespan_2 (Default|GetEarliestMention (Utilities|Array|Get(acopy) _output_get _index)))
          (if (> _timespan_2 _timespan)
            (Utilities|Array|Swap _output_get _index_2 _index)))))
    (:then_1
      ;[0 0 0] Find most mentioned concept time
      (for _array_element (LocalVariables|GetLocal_SortedConcepts)
        (bind _totalseconds (Default|GetTotalMention _array_element))
        (if (> _totalseconds (LocalVariables|GetLocal_BiggestConcept))
          (LocalVariables|SetLocal_BiggestConcept _totalseconds))))
    (:then_2
      ;[0 0 0] Reposition concept on XYZ coordinates
      (for (_array_element_2 _array_index) (LocalVariables|GetLocal_SortedConcepts)
        (bind _totalseconds_2 (Default|GetTotalMention _array_element_2))
        (Transformation|SetActorLocation _array_element_2 (Math|Vector|MakeVector (- (+ (.x _origin) (.x _boxextent)) (* _array_index (/ (* (.x _boxextent) 2.0) (Utilities|Array|Length (LocalVariables|GetLocal_SortedConcepts))))) (+ (- (.y _origin) (.y _boxextent)) (* (* (.y _boxextent) 2.0) (Math|Float|SafeDivide (* (Math|Float|Absolute(Float) (- (Math|Integer|%(Integer) _array_index (- _returnvalue_2 2)) (/ _returnvalue_3 2.0))) 2.0) _returnvalue_3))) (Math|Float|Lerp _returnvalue_4 (+ _returnvalue_4 (* (.z _boxextent) 2.0)) (Math|Float|SafeDivide _totalseconds_2 (LocalVariables|GetLocal_BiggestConcept)))) false true)))))