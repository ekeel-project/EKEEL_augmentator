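; BP_HighlighterVisualiser drives mention highlighting and visibility of spawned concept and link actors as media plays.
; Once the Spawner completes, it caches both actor sets and binds handlers to MediaPlayer seek events, gated by highlighter and visualiser toggles.
; Seek time and media ID are matched against annotation ranges and link timestamps to set mention flags.
; Concepts then update highlights, while concepts and links update visibility.
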(event Custom|LoadData
  (bind _logger (Variables|Default|GetLogger))
  (bind _logger_2 (Variables|Default|GetLogger))
  (bind _logger_3 (Variables|Default|GetLogger))
  (Utilities|FlowControl|Sequence
    (:then_0
      ;[1 1 1] Obtain concept and link actors
      (Utilities|FlowControl|Sequence
        (:then_0
          (bind _conceptactors (Default|GetConceptActorMap (Variables|Default|GetSpawner)))
          (bind _values (Utilities|Map|Values _conceptactors))
          (Variables|Default|SetConceptActors _values))
        (:then_1
          (bind _linkactors (Default|GetLinkActorMap (Variables|Default|GetSpawner)))
          (bind _values_2 (Utilities|Map|Values _linkactors))
          (Variables|Default|SetLinkActors _values_2))
        (:then_2
          ;;[0.4778 1 0] Log when highlighter and visualiser obtains actors
          (Utilities|IsValid _logger_3
            (:Is%20Valid
              (Default|Log _logger_3 "HigVis" "Log" "Obtained concept and link actors." (Variables|Default|GetLog)))))))
    (:then_1
      (if (or (Variables|Default|GetEnableHighlighter) (Variables|Default|GetEnableVisualiser))
        (EventDispatchers|BindEventtoSeekFire (Variables|Default|GetMedia%20Player) (delegate Custom|UpdateMentions))
        ;[1 1 1] Update highlights
        (if (Variables|Default|GetEnableHighlighter)
          (Utilities|FlowControl|Sequence
            (:then_0
              ;;[0.4778 1 0] Log if highlighter is enabled
              (Utilities|IsValid _logger
                (:Is%20Valid
                  (Default|Log _logger "HigVis" "Log" "Highlighter enabled." (Variables|Default|GetLog)))))
            (:then_1
              (EventDispatchers|BindEventtoSeekFire (Variables|Default|GetMedia%20Player) (delegate Custom|UpdateHighlight))
              ;[1 1 1] Update visibility
              (if (Variables|Default|GetEnableVisualiser) :!label _label
                (Utilities|FlowControl|Sequence
                  (:then_0
                    ;;[0.4778 1 0] Log if visualiser is enabled
                    (Utilities|IsValid _logger_2
                      (:Is%20Valid
                        (Default|Log _logger_2 "HigVis" "Log" "Visualiser enabled." (Variables|Default|GetLog)))))
                  (:then_1
                    (EventDispatchers|BindEventtoSeekFire (Variables|Default|GetMedia%20Player) (delegate Custom|UpdateVisibility)))))))
          (else
            (goto _label)))))))

(event Custom|UpdateHighlight
  (params (SeekTime :type Timespan%20Structure) (Duration :type Timespan%20Structure) (MediaID :type String))
  ;[1 1 1] Update highlights
  (for _array_element (Variables|Default|GetConceptActors)
    (Default|UpdateHighlight _array_element)))

(event Custom|UpdateVisibility
  (params (SeekTime :type Timespan%20Structure) (Duration :type Timespan%20Structure) (MediaID :type String))
  ;[1 1 1] Update visibility
  (Utilities|FlowControl|Sequence
    (:then_0
      (for _array_element (Variables|Default|GetConceptActors)
        (Default|UpdateVisibility _array_element)))
    (:then_1
      (for _array_element_2 (Variables|Default|GetLinkActors)
        (Default|UpdateVisibility _array_element_2)))))

(event Custom|UpdateMentions
  (params (SeekTime :type Timespan%20Structure) (Duration :type Timespan%20Structure) (MediaID :type String))
  ;[0 0 0] Update mentions
  ;;[1 1 1] Update Concept Mentions
  (Utilities|FlowControl|Sequence
    (:then_0
      (for _array_element (Variables|Default|GetConceptActors)
        (bind _annotationsdata (Default|GetAnnotationsData _array_element))
        (bind _array_element_2 (Utilities|Array|ForEachLoopwithBreak _annotationsdata :!label _label)
          (:LoopBody
            (if (Math|Boolean|ANDBoolean (Utilities|Enum|Equal(Enum) (.source (Utilities|Struct|BreakS_ConceptAnnotation _array_element_2)) MediaID) (>= SeekTime (.start_timestamp (Utilities|Struct|BreakS_ConceptAnnotation _array_element_2))) (<= SeekTime (.end_timestamp (Utilities|Struct|BreakS_ConceptAnnotation _array_element_2))))
              (Variables|/Game/Blueprints/BP_Concept.BP_Concept_C|SetisMentioned _array_element true)
              (Variables|/Game/Blueprints/BP_Concept.BP_Concept_C|SetbeenMentioned _array_element true)
              (goto _label Break)
              (else
                (Variables|/Game/Blueprints/BP_Concept.BP_Concept_C|SetisMentioned _array_element false)))))))
    (:then_1
      ;;[1 1 1] Update Link Mention
      (for _array_element_3 (Variables|Default|GetLinkActors)
        (bind _linkdata (Default|GetLinkData _array_element_3))
        (if (and (Utilities|Enum|Equal(Enum) (.source (Utilities|Struct|BreakS_Link _linkdata)) MediaID) (>= SeekTime (.timestamp (Utilities|Struct|BreakS_Link _linkdata))))
          (Variables|/Game/Blueprints/BP_Link.BP_Link_C|SetbeenMentioned _array_element_3 true))))))

(event EventBeginPlay
  ;[0 1 0.01177] Initial checks
  (Utilities|FlowControl|Sequence
    (:then_0
      (if (and (not (Utilities|IsValid (Variables|Default|GetLogger))) (Variables|Default|GetLog))
        (Development|PrintString "[Warning][HigVis] Logging enabled but no Logger specified.")))
    (:then_1
      (Utilities|IsValid (Variables|Default|GetSpawner)
        (:Is%20Not%20Valid
          (Development|PrintString "[Warning][HigVis] Missing a ConceptLinkArea."))))
    (:then_2
      (Utilities|IsValid (Variables|Default|GetSpawner)
        (:Is%20Valid
          (Utilities|IsValid (Variables|Default|GetMedia%20Player)
            (:Is%20Valid
              (EventDispatchers|BindEventtoSpawnComplete (Variables|Default|GetSpawner) (delegate Custom|LoadData)))))))))

(event Collision|EventActorBeginOverlap
  (params (OtherActor :type Actor%20Object%20Reference)))

(event EventTick
  (params (DeltaSeconds :type Float%20%28single-precision%29)))

(fn ConstructionScript)

(fn ConfigureParameters
  (params (EnableHighlighter :type Boolean) (EnableVisualiser :type Boolean))
  (Utilities|FlowControl|Sequence
    (:then_0
      (Variables|Default|SetEnableHighlighter EnableHighlighter))
    (:then_1
      (Variables|Default|SetEnableVisualiser EnableVisualiser))))