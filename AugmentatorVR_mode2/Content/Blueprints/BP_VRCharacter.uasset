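; VR player character for exploring a concept map: teleporting, grabbing, linking concepts and playing media annotations.
; Tick recenters the character under the headset and tracks each hand's nearest grabbable, which feeds grabs, links, highlights and the active annotation menu.
; Drawn links reveal matching existing links or turn red before timed deletion.
; Teleports use Niagara-drawn, navmesh-projected arcs, a sphere toggles camera-facing labels, and interactions report to a Logger.
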(event OnComponentBeginOverlap(TextSphere)
  (params (OverlappedComponent :type Primitive%20Component%20Object%20Reference) (OtherActor :type Actor%20Object%20Reference) (OtherComp :type Primitive%20Component%20Object%20Reference) (OtherBodyIndex :type Integer) (bFromSweep :type Boolean) (SweepResult :type Hit%20Result%20Structure%20%28by%20ref%29))
  ;[0 0 0] UPDATES
  ; Events used to repeatedly perform updates and execute functions related to
  ; overlap events.
  ;;[1 1 1] TEXT ROTATION
  (Utilities|FlowControl|Sequence
    (:then_0
      (bind _asbp_concept (Utilities|Casting|CastToBP_Concept OtherActor))
      (Default|EnableLabelRotation _asbp_concept (Variables|Default|GetCamera)))
    (:then_1
      (bind _asbp_link (Utilities|Casting|CastToBP_Link OtherActor))
      (Default|EnableLabelRotation _asbp_link (Variables|Default|GetCamera)))))

(event OnComponentEndOverlap(TextSphere)
  (params (OverlappedComponent :type Primitive%20Component%20Object%20Reference) (OtherActor :type Actor%20Object%20Reference) (OtherComp :type Primitive%20Component%20Object%20Reference) (OtherBodyIndex :type Integer))
  ;[0 0 0] UPDATES
  ; Events used to repeatedly perform updates and execute functions related to
  ; overlap events.
  ;;[1 1 1] TEXT ROTATION
  (Utilities|FlowControl|Sequence
    (:then_0
      (bind _asbp_concept (Utilities|Casting|CastToBP_Concept OtherActor))
      (Default|DisableLabelRotation _asbp_concept))
    (:then_1
      (bind _asbp_link (Utilities|Casting|CastToBP_Link OtherActor))
      (Default|DisableLabelRotation _asbp_link))))

(event Custom|PlayAnnotation
  (bind _logger (Variables|Default|GetLogger))
  ;[0 0 0] INTERACTIONS
  ; Input actions used to perform interactions by the character class
  ; with the other actors within the level it is located in.
  ;;[1 1 1] ANNOTATION ACTIONS
  (bind _annotationmenu (Variables|Default|GetAnnotationMenu)
    (:then
      (bind (_valid _annotationdata) (Default|GetSelectedAnnotation _annotationmenu))
      (if _valid ; If the selected annotation exist\nplay it on the media player
        (bind _mediaplayer (Variables|Default|GetMediaPlayer)
          (:then
            (Default|PlayMedia _mediaplayer (.source (Utilities|Struct|BreakS_ConceptAnnotation _annotationdata)) (Utilities|Struct|MakeMediaPlayerOptions "(Audio=0,Caption=-1,Metadata=-1,Script=-1,Subtitle=-1,Text=-1,Video=0)" (.start_timestamp (Utilities|Struct|BreakS_ConceptAnnotation _annotationdata)) "Enabled" "Disabled"))
            ;;;[0.1677 1 0] Log: Play annotation
            (Utilities|IsValid _logger
              (:Is%20Valid
                (Default|LogAction _logger "NewEnumerator9" (.ann_id (Utilities|Struct|BreakS_ConceptAnnotation _annotationdata)) "" (Variables|Default|GetLog)))))
          (:else))))
    (:else)))

(event Input|EnhancedActionEvents|EnhancedInputActionIA_CreateLinkLeft
  (params (ActionValue :type Boolean) (ElapsedSeconds :type Float%20%28double-precision%29) (TriggeredSeconds :type Float%20%28double-precision%29) (InputAction :type Input%20Action%20Object%20Reference :default "/Game/Inputs/IA_CreateLinkLeft.IA_CreateLinkLeft"))
  (bind _logger (Variables|Default|GetLogger))
  (bind _logger_2 (Variables|Default|GetLogger))
  ;[0 0 0] INTERACTIONS
  ; Input actions used to perform interactions by the character class
  ; with the other actors within the level it is located in.
  ;;[1 1 1] CREATE LINK ACTIONS
  (:Started
    (if (Variables|Default|GetAllowLinkCreate)
      (bind (_valid _link _startpoint) (CallFunction|StartLinkAction "NewEnumerator1"))
      (if _valid ; Log concept as starting point
        (bind _conceptdata (Default|GetConceptData _startpoint)))
      ;;;[0.1677 1 0] Log: Create link start action
      (Utilities|IsValid _logger_2
        (:Is%20Valid
          (Default|LogAction _logger_2 "NewEnumerator14" (select _valid (.id (Utilities|Struct|BreakS_Concept _conceptdata)) "") "L" (Variables|Default|GetLog))))))
  (:Completed
    (if (Variables|Default|GetAllowLinkCreate)
      (bind (_valid_2 _endpoint) (CallFunction|ConnectandValidateLink _link _startpoint "NewEnumerator1"))
      (if _valid_2 ; Log concept as ending point
        (bind _conceptdata_2 (Default|GetConceptData _endpoint)))
      ;;;[0.1677 1 0] Log: Create link end action
      (Utilities|IsValid _logger
        (:Is%20Valid
          (Default|LogAction _logger "NewEnumerator15" (select _valid_2 (.id (Utilities|Struct|BreakS_Concept _conceptdata_2)) "") "L" (Variables|Default|GetLog)))))))

(event Input|EnhancedActionEvents|EnhancedInputActionIA_CreateLinkRight
  (params (ActionValue :type Boolean) (ElapsedSeconds :type Float%20%28double-precision%29) (TriggeredSeconds :type Float%20%28double-precision%29) (InputAction :type Input%20Action%20Object%20Reference :default "/Game/Inputs/IA_CreateLinkRight.IA_CreateLinkRight"))
  (bind _logger (Variables|Default|GetLogger))
  (bind _logger_2 (Variables|Default|GetLogger))
  ;[0 0 0] INTERACTIONS
  ; Input actions used to perform interactions by the character class
  ; with the other actors within the level it is located in.
  ;;[1 1 1] CREATE LINK ACTIONS
  (:Started
    (if (Variables|Default|GetAllowLinkCreate)
      (bind (_valid _link _startpoint) (CallFunction|StartLinkAction "NewEnumerator0"))
      (if _valid ; Log concept as starting point
        (bind _conceptdata (Default|GetConceptData _startpoint)))
      ;;;[0.1677 1 0] Log: Create link start action
      (Utilities|IsValid _logger
        (:Is%20Valid
          (Default|LogAction _logger "NewEnumerator14" (select _valid (.id (Utilities|Struct|BreakS_Concept _conceptdata)) "") "R" (Variables|Default|GetLog))))))
  (:Completed
    (if (Variables|Default|GetAllowLinkCreate)
      (bind (_valid_2 _endpoint) (CallFunction|ConnectandValidateLink _link _startpoint "NewEnumerator0"))
      (if _valid_2 ; Log concept as ending point
        (bind _conceptdata_2 (Default|GetConceptData _endpoint)))
      ;;;[0.1677 1 0] Log: Create link end action
      (Utilities|IsValid _logger_2
        (:Is%20Valid
          (Default|LogAction _logger_2 "NewEnumerator15" (select _valid_2 (.id (Utilities|Struct|BreakS_Concept _conceptdata_2)) "") "R" (Variables|Default|GetLog)))))))

(event Input|EnhancedActionEvents|EnhancedInputActionIA_GrabRight
  (params (ActionValue :type Boolean) (ElapsedSeconds :type Float%20%28double-precision%29) (TriggeredSeconds :type Float%20%28double-precision%29) (InputAction :type Input%20Action%20Object%20Reference :default "/Game/Inputs/IA_GrabRight.IA_GrabRight"))
  (bind _logger (Variables|Default|GetLogger))
  (bind _logger_2 (Variables|Default|GetLogger))
  ;[0 0 0] INTERACTIONS
  ; Input actions used to perform interactions by the character class
  ; with the other actors within the level it is located in.
  ;;[1 1 1] GRAB ACTIONS
  (:Started
    (bind (_valid _grabbedactor) (CallFunction|StartGrabAction "NewEnumerator0"))
    (bind _asbp_concept (Utilities|Casting|CastToBP_Concept _grabbedactor)
      (:then
        (bind _conceptdata (Default|GetConceptData _asbp_concept)))
      (:CastFailed
        _))
    ;;;[0.1677 1 0] Log: Grab action
    (Utilities|IsValid _logger
      (:Is%20Valid
        (Default|LogAction _logger "NewEnumerator0" (select _valid (.id (Utilities|Struct|BreakS_Concept _conceptdata)) "") "R" (Variables|Default|GetLog)))))
  (:Completed
    (bind (_valid_2 _releasedactor) (CallFunction|CompleteGrabAction "NewEnumerator0"))
    (bind _asbp_concept_2 (Utilities|Casting|CastToBP_Concept _releasedactor)
      (:then
        (bind _conceptdata_2 (Default|GetConceptData _asbp_concept_2)))
      (:CastFailed
        _))
    ;;;[0.1677 1 0] Log: Release action
    (Utilities|IsValid _logger_2
      (:Is%20Valid
        (Default|LogAction _logger_2 "NewEnumerator1" (select _valid_2 (.id (Utilities|Struct|BreakS_Concept _conceptdata_2)) "") "R" (Variables|Default|GetLog))))))

(event Input|EnhancedActionEvents|EnhancedInputActionIA_GrabLeft
  (params (ActionValue :type Boolean) (ElapsedSeconds :type Float%20%28double-precision%29) (TriggeredSeconds :type Float%20%28double-precision%29) (InputAction :type Input%20Action%20Object%20Reference :default "/Game/Inputs/IA_GrabLeft.IA_GrabLeft"))
  (bind _logger (Variables|Default|GetLogger))
  (bind _logger_2 (Variables|Default|GetLogger))
  ;[0 0 0] INTERACTIONS
  ; Input actions used to perform interactions by the character class
  ; with the other actors within the level it is located in.
  ;;[1 1 1] GRAB ACTIONS
  (:Started
    (bind (_valid _grabbedactor) (CallFunction|StartGrabAction "NewEnumerator1"))
    (bind _asbp_concept (Utilities|Casting|CastToBP_Concept _grabbedactor)
      (:then
        (bind _conceptdata (Default|GetConceptData _asbp_concept)))
      (:CastFailed
        _))
    ;;;[0.1677 1 0] Log: Grab action
    (Utilities|IsValid _logger
      (:Is%20Valid
        (Default|LogAction _logger "NewEnumerator0" (select _valid (.id (Utilities|Struct|BreakS_Concept _conceptdata)) "") "L" (Variables|Default|GetLog)))))
  (:Completed
    (bind (_valid_2 _releasedactor) (CallFunction|CompleteGrabAction "NewEnumerator1"))
    (bind _asbp_concept_2 (Utilities|Casting|CastToBP_Concept _releasedactor)
      (:then
        (bind _conceptdata_2 (Default|GetConceptData _asbp_concept_2)))
      (:CastFailed
        _))
    ;;;[0.1677 1 0] Log: Release action
    (Utilities|IsValid _logger_2
      (:Is%20Valid
        (Default|LogAction _logger_2 "NewEnumerator1" (select _valid_2 (.id (Utilities|Struct|BreakS_Concept _conceptdata_2)) "") "L" (Variables|Default|GetLog))))))

(event Input|EnhancedActionEvents|EnhancedInputActionIA_PlayAnnotation
  (params (ActionValue :type Boolean) (ElapsedSeconds :type Float%20%28double-precision%29) (TriggeredSeconds :type Float%20%28double-precision%29) (InputAction :type Input%20Action%20Object%20Reference :default "/Game/Inputs/IA_PlayAnnotation.IA_PlayAnnotation"))
  (bind _logger (Variables|Default|GetLogger))
  ;[0 0 0] INTERACTIONS
  ; Input actions used to perform interactions by the character class
  ; with the other actors within the level it is located in.
  ;;[1 1 1] ANNOTATION ACTIONS
  (:Completed
    (bind _annotationmenu (Variables|Default|GetAnnotationMenu)
      (:then
        (bind (_valid _annotationdata) (Default|GetSelectedAnnotation _annotationmenu))
        (if _valid ; If the selected annotation exist\nplay it on the media player
          (bind _mediaplayer (Variables|Default|GetMediaPlayer)
            (:then
              (Default|PlayMedia _mediaplayer (.source (Utilities|Struct|BreakS_ConceptAnnotation _annotationdata)) (Utilities|Struct|MakeMediaPlayerOptions "(Audio=0,Caption=-1,Metadata=-1,Script=-1,Subtitle=-1,Text=-1,Video=0)" (.start_timestamp (Utilities|Struct|BreakS_ConceptAnnotation _annotationdata)) "Enabled" "Disabled"))
              ;;;[0.1677 1 0] Log: Play annotation
              (Utilities|IsValid _logger
                (:Is%20Valid
                  (Default|LogAction _logger "NewEnumerator9" (.ann_id (Utilities|Struct|BreakS_ConceptAnnotation _annotationdata)) "" (Variables|Default|GetLog)))))
            (:else))))
      (:else))))

(event Input|EnhancedActionEvents|EnhancedInputActionIA_SelectEntry
  (params (ActionValue :type Float%20%28double-precision%29) (ElapsedSeconds :type Float%20%28double-precision%29) (TriggeredSeconds :type Float%20%28double-precision%29) (InputAction :type Input%20Action%20Object%20Reference :default "/Game/Inputs/IA_SelectEntry.IA_SelectEntry"))
  (bind _annotationmenu (Variables|Default|GetAnnotationMenu))
  ;[0 0 0] INTERACTIONS
  ; Input actions used to perform interactions by the character class
  ; with the other actors within the level it is located in.
  ;;[1 1 1] ANNOTATION ACTIONS
  (Variables|Default|GetAnnotationMenu
    (:then
      (if (> ActionValue 0.0)
        (Default|SelectUp _annotationmenu)
        (else
          (Default|SelectDown _annotationmenu))))
    (:else)))

(event Input|EnhancedActionEvents|EnhancedInputActionIA_TeleportLeft
  (params (ActionValue :type Boolean) (ElapsedSeconds :type Float%20%28double-precision%29) (TriggeredSeconds :type Float%20%28double-precision%29) (InputAction :type Input%20Action%20Object%20Reference :default "/Game/Inputs/IA_TeleportLeft.IA_TeleportLeft"))
  (bind _logger (Variables|Default|GetLogger))
  ;[0 0 0] INTERACTIONS
  ; Input actions used to perform interactions by the character class
  ; with the other actors within the level it is located in.
  ;;[1 1 1] TELEPORT ACTIONS
  (:Triggered
    (CallFunction|UpdateTeleportAction (stale _trace) (stale _marker) (Variables|Default|GetMotionControllerAimL)))
  (:Started
    (bind (_trace _marker) (CallFunction|StartTeleportAction (Variables|Default|GetMotionControllerAimL))))
  (:Completed
    (bind _success (CallFunction|CompleteTeleportAction _trace _marker (Variables|Default|GetMotionControllerAimL)))
    (if _success
      ;;;[0.1677 1 0] Log: Teleport action
      (Utilities|IsValid _logger
        (:Is%20Valid
          (Default|LogAction _logger "NewEnumerator2" "" "L" (Variables|Default|GetLog)))))))

(event Input|EnhancedActionEvents|EnhancedInputActionIA_TeleportRight
  (params (ActionValue :type Boolean) (ElapsedSeconds :type Float%20%28double-precision%29) (TriggeredSeconds :type Float%20%28double-precision%29) (InputAction :type Input%20Action%20Object%20Reference :default "/Game/Inputs/IA_TeleportRight.IA_TeleportRight"))
  (bind _logger (Variables|Default|GetLogger))
  ;[0 0 0] INTERACTIONS
  ; Input actions used to perform interactions by the character class
  ; with the other actors within the level it is located in.
  ;;[1 1 1] TELEPORT ACTIONS
  (:Triggered
    (CallFunction|UpdateTeleportAction (stale _trace) (stale _marker) (Variables|Default|GetMotionControllerAimR)))
  (:Started
    (bind (_trace _marker) (CallFunction|StartTeleportAction (Variables|Default|GetMotionControllerAimR))))
  (:Completed
    (bind _success (CallFunction|CompleteTeleportAction _trace _marker (Variables|Default|GetMotionControllerAimR)))
    (if _success
      ;;;[0.1677 1 0] Log: Teleport action
      (Utilities|IsValid _logger
        (:Is%20Valid
          (Default|LogAction _logger "NewEnumerator2" "" "R" (Variables|Default|GetLog)))))))

(event Input|EnhancedActionEvents|EnhancedInputActionIA_TogglePlayback
  (params (ActionValue :type Boolean) (ElapsedSeconds :type Float%20%28double-precision%29) (TriggeredSeconds :type Float%20%28double-precision%29) (InputAction :type Input%20Action%20Object%20Reference :default "/Game/Inputs/IA_TogglePlayback.IA_TogglePlayback"))
  (bind _logger (Variables|Default|GetLogger))
  (bind _logger_2 (Variables|Default|GetLogger))
  (bind _logger_3 (Variables|Default|GetLogger))
  ;[0 0 0] INTERACTIONS
  ; Input actions used to perform interactions by the character class
  ; with the other actors within the level it is located in.
  ;;[1 1 1] ANNOTATION ACTIONS
  (:Completed
    (Variables|Default|GetMediaPlayer
      (:then
        (if (< ElapsedSeconds (Variables|Default|GetButtonHoldThreshold))
          (bind _isplaying (Default|GetPlayStatus (Variables|Default|GetMediaPlayer)))
          (if _isplaying
            (Default|PauseMedia (Variables|Default|GetMediaPlayer))
            ;;;[0.1677 1 0] Log: Pause media
            (Utilities|IsValid _logger_3
              (:Is%20Valid
                (Default|LogAction _logger_3 "NewEnumerator11" "" "" (Variables|Default|GetLog))))
            (else
              (Default|ResumeMedia (Variables|Default|GetMediaPlayer))
              ;;;[0.1677 1 0] Log: Resume media
              (Utilities|IsValid _logger
                (:Is%20Valid
                  (Default|LogAction _logger "NewEnumerator10" "" "" (Variables|Default|GetLog))))))
          (else
            (bind _mediamap (Default|GetMediaMap (Variables|Default|GetMediaPlayer)))
            (bind _keys (Utilities|Map|Keys _mediamap))
            (Default|PlayMedia (Variables|Default|GetMediaPlayer) (Utilities|Array|Get(acopy) _keys) (Utilities|Struct|MakeMediaPlayerOptions "(Audio=0,Caption=-1,Metadata=-1,Script=-1,Subtitle=-1,Text=-1,Video=0)" "+00000000.00:00:00.000000000" "Enabled" "Disabled"))
            ;;;[0.1677 1 0] Log: Play media
            (Utilities|IsValid _logger_2
              (:Is%20Valid
                (Default|LogAction _logger_2 "NewEnumerator16" (Utilities|Array|Get(acopy) _keys) "" (Variables|Default|GetLog)))))))
      (:else))))

(event EventBeginPlay
  (bind _logger (Variables|Default|GetLogger))
  ;[0 0 0] INITIALISATION
  ; Events used for initialisation purposes of the module and binding to other modules
  ; to request data when it has been successfully created.
  ;;[1 1 1] BEGINPLAY
  (Utilities|FlowControl|Sequence
    (:then_0
      (if (and (not (Utilities|IsValid (Variables|Default|GetLogger))) (Variables|Default|GetLog))
        (Development|PrintString "[Warning][VRCharacter] Logging enabled but no Logger specified.")))
    (:then_1
      (Utilities|IsValid (Variables|Default|GetMediaPlayer) ; Media player warning
        (:Is%20Not%20Valid
          (Development|PrintString "[Warning][VRCharacter] Media Player not specified."))))
    (:then_2
      (Class|HeadMountedDisplayFunctionLibrary|SetTrackingOrigin "Stage")
      (bind _asplayer_controller (Utilities|Casting|CastToPlayerController (Pawn|GetController)))
      (Input|AddMappingContext (PlayerController|LocalPlayerSubsystems|GetEnhancedInputLocalPlayerSubsystem _asplayer_controller) "/Game/Inputs/IMC_Controls.IMC_Controls" 1 "(bIgnoreAllPressedKeysUntilRelease=True,bForceImmediately=False,bNotifyUserSettings=False)") ; Set control mapping to player controller
    )
    (:then_3
      (Class|HeadMountedDisplayFunctionLibrary|ResetOrientationandPosition 0.0 "OrientationAndPosition")
      (Development|ExecuteConsoleCommand "vr.PixelDensity 1.0" 0)
      ;;;[0.1677 1 0] Log: VRCharacter initialised
      (Utilities|IsValid _logger
        (:Is%20Valid
          (Default|Log _logger "VRCharacter" "Log" "Character initialised" (Variables|Default|GetLog)))))))

(event EventTick
  (params (DeltaSeconds :type Float%20%28single-precision%29))
  (bind _returnvalue (Transformation|GetActorLocation))
  (bind _camera (Variables|Default|GetCamera))
  (bind _returnvalue_2 (Transformation|GetWorldLocation _camera))
  (bind _returnvalue_3 (- _returnvalue_2 _returnvalue))
  (bind (_x _y) (Math|Vector|BreakVector _returnvalue_3))
  (bind _returnvalue_4 (Math|Vector|NegateVector _returnvalue_3))
  ;[0 0 0] UPDATES
  ; Events used to repeatedly perform updates and execute functions related to
  ; overlap events.
  ;;[1 1 1] TICK
  (Utilities|FlowControl|Sequence
    (:then_0
      (Variables|Default|GetHeldComponentR
        (:then)
        (:else
          (bind _grabbableactor (CallFunction|GetNearestGrabbable (Variables|Default|GetMotionControllerR) (Variables|Default|GetGrabRadius)))
          (CallFunction|UpdateTouchedActor _grabbableactor "NewEnumerator0"))))
    (:then_1
      (Variables|Default|GetHeldComponentL
        (:then)
        (:else
          (bind _grabbableactor_2 (CallFunction|GetNearestGrabbable (Variables|Default|GetMotionControllerL) (Variables|Default|GetGrabRadius)))
          (CallFunction|UpdateTouchedActor _grabbableactor_2 "NewEnumerator1"))))
    (:then_2
      (Class|MovementComponent|MoveUpdatedComponent (Variables|Character|GetCharacterMovement) (Math|Vector|MakeVector _x _y 0.0) (Transformation|GetActorRotation) true)
      (Transformation|AddWorldOffset (Variables|Default|GetVROrigin) (Math|Vector|MakeVector (.x _returnvalue_4) (.y _returnvalue_4) 0.0) false false))))

(fn ConstructionScript
  (Components|Sphere|SetSphereRadius (Variables|Default|GetTextSphere) (Variables|Default|GetCollisionSphereRadius) true))

(fn GetNearestGrabbable
  (params (MotionController :type Motion%20Controller%20Component%20Object%20Reference) (WithinRange :type Float%20%28double-precision%29))
  (bind _returnvalue (Transformation|GetWorldLocation MotionController))
  (bind (_outactors _returnvalue_2) (Collision|SphereOverlapActors _returnvalue WithinRange (Utilities|Array|MakeArray "ObjectTypeQuery7") 0 :!pinned true)) ; Trace for grabbable actors within a range
  (if _returnvalue_2
    (return (.ReturnValue (Actor|FindNearestActor _returnvalue _outactors)))
    (else
      (return 0))))

(fn ComputeTeleportArc
  (params (MotionController :type Motion%20Controller%20Component%20Object%20Reference))
  (bind (_outhit _outpathpositions) (Class|GameplayStatics|BlueprintPredictProjectilePathbyTraceChannel (Transformation|GetWorldLocation MotionController) (* (Math|Vector|GetForwardVector MotionController) 5e+02) true 0.0 "ECC_WorldStatic" false (Utilities|Array|MakeArray self) "None")) ; Predict a path from motion controller with\nsame direction
  (return (.ReturnValue (AI|Navigation|ProjectPointtoNavigation (.Location (Collision|BreakHitResult _outhit)) 0 0 "0, 0, 0")) (.ProjectedLocation (AI|Navigation|ProjectPointtoNavigation (.Location (Collision|BreakHitResult _outhit)) 0 0 "0, 0, 0")) _outpathpositions))

(fn UpdateTouchedActor
  (params (Actor :type Actor%20Object%20Reference) (HandType :type HandType%20Enum :default "NewEnumerator0"))
  (bind _logger (Variables|Default|GetLogger))
  (if (!= Actor (Utilities|Select :Index HandType :NewEnumerator0 (Variables|Default|GetTouchedActorR) :NewEnumerator1 (Variables|Default|GetTouchedActorL))) ; Update touched actor only if \nthe newly touched actor is different
    (Utilities|FlowControl|Sequence
      (:then_0
        (bind _asbp_concept (Utilities|Casting|CastToBP_Concept (Utilities|Select :Index HandType :NewEnumerator0 (Variables|Default|GetTouchedActorR) :NewEnumerator1 (Variables|Default|GetTouchedActorL)) :!pinned true)) ; Old touched was a concept
        (if (!= _asbp_concept (Utilities|Select :Index HandType :NewEnumerator0 (Variables|Default|GetTouchedActorL) :NewEnumerator1 (Variables|Default|GetTouchedActorR))) ; Unfocus concept if is isnt touched\nby the other controller
          (Variables|/Game/Blueprints/BP_Concept.BP_Concept_C|SetisFocused _asbp_concept false)
          (Default|UpdateHighlight _asbp_concept)))
      (:then_1
        (bind _asbp_concept_2 (Utilities|Casting|CastToBP_Concept Actor :!pinned true)) ; New touched is a concept
        (Variables|/Game/Blueprints/BP_Concept.BP_Concept_C|SetisFocused _asbp_concept_2 true)
        (Default|UpdateHighlight _asbp_concept_2)
        (Default|OpenMenu _asbp_concept_2) ; Automatically open concept menu
        (Utilities|FlowControl|Sequence
          (:then_0
            (bind _conceptdata (Default|GetConceptData _asbp_concept_2)) ; Log action when touching a new concept
            ;[0.1677 1 0] Log: Touched concept
            (Utilities|IsValid _logger
              (:Is%20Valid
                (Default|LogAction _logger "NewEnumerator3" (.id (Utilities|Struct|BreakS_Concept _conceptdata)) (Utilities|Select :Index HandType :NewEnumerator0 "R" :NewEnumerator1 "L") (Variables|Default|GetLog)))))
          (:then_1
            (bind _annotationmenu (Default|GetAnnotationMenu _asbp_concept_2))
            (Utilities|IsValid _annotationmenu
              (:Is%20Valid
                (bind _annotationmenu_2 (Default|GetAnnotationMenuWidget _annotationmenu)) ; Retrieve the annotation menu
                (Variables|Default|SetAnnotationMenu _annotationmenu_2))
              (:Is%20Not%20Valid
                (Variables|Default|SetAnnotationMenu 0))))))
      (:then_2
        (Utilities|IsValid Actor :!pinned true ; Play haptic if touched a valid actor
          (:Is%20Valid
            (Class|PlayerController|PlayHapticEffect (Game|GetPlayerController 0) "/Game/Haptics/HF_ShortHaptic.HF_ShortHaptic" (Utilities|Select :Index HandType :NewEnumerator0 "Right" :NewEnumerator1 "Left") 1.0 false))))
      (:then_3
        (switch Utilities|FlowControl|Switch|SwitchonHandType HandType ; Update actor reference
          (:NewEnumerator0
            (Variables|Default|SetTouchedActorR Actor))
          (:NewEnumerator1
            (Variables|Default|SetTouchedActorL Actor)))))))

(fn StartTeleportAction
  (params (MotionController :type Motion%20Controller%20Component%20Object%20Reference))
  (Utilities|FlowControl|Sequence
    (:then_0
      (bind _returnvalue (Niagara|SpawnSystemAttached "/Game/FX/NS_TeleportTrace.NS_TeleportTrace" MotionController "None" "0, 0, 0" "0, 0, 0" "KeepRelativeOffset" true :!pinned true)) ; Initialise Trace niagara
      (Niagara|SetNiagaraVariable(LinearColor) _returnvalue "User.Colour" (Variables|Default|GetTeleportColour)))
    (:then_1
      (bind _returnvalue_2 (Niagara|SpawnSystematLocation "/Game/FX/NS_TeleportMarker.NS_TeleportMarker" "0, 0, 0" :!pinned true)) ; Initialise Marker niagara
      (Niagara|SetNiagaraVariable(LinearColor) _returnvalue_2 "User.Colour" (Variables|Default|GetTeleportColour)))
    (:then_2
      (return _returnvalue _returnvalue_2))))

(fn UpdateTeleportAction
  (params (Trace :type Niagara%20Component%20Object%20Reference) (Marker :type Niagara%20Component%20Object%20Reference) (MotionController :type Motion%20Controller%20Component%20Object%20Reference))
  (bind (_isvalid _teleportposition _outpathpositions) (CallFunction|ComputeTeleportArc MotionController :!pinned true)) ; Update and find validity of teleport position
  (Utilities|FlowControl|Sequence
    (:then_0
      (Class|NiagaraDataInterfaceArrayFunctionLibrary|SetNiagaraArrayVector Trace "User.ParticlePath" _outpathpositions :!pinned true) ; Update arc points
    )
    (:then_1
      (Transformation|SetWorldLocation Marker _teleportposition false true :!pinned true) ; Update marker location and visibility
      (Rendering|SetVisibility Marker _isvalid false))))

(fn CompleteTeleportAction
  (params (Trace :type Niagara%20Component%20Object%20Reference) (Marker :type Niagara%20Component%20Object%20Reference) (MotionController :type Motion%20Controller%20Component%20Object%20Reference))
  (Utilities|FlowControl|Sequence
    (:then_0
      (Components|DestroyComponent Trace :!pinned true) ; Destroy niagara visualising teleport
      (Components|DestroyComponent Marker))
    (:then_1
      (bind (_isvalid _teleportposition) (CallFunction|ComputeTeleportArc MotionController))
      (if _isvalid ; Compute teleport and teleport if valid
        (bind _returnvalue (Transformation|Teleport _teleportposition "0, 0, 0"))
        (return _returnvalue)
        (else
          (return false))))))

(fn StartGrabAction
  (params (HandType :type HandType%20Enum :default "NewEnumerator0"))
  (bind _touchedactorr (Variables|Default|GetTouchedActorR))
  (bind _touchedactorl (Variables|Default|GetTouchedActorL))
  (bind _returnvalue (Utilities|Select :Index HandType :NewEnumerator0 _touchedactorr :NewEnumerator1 _touchedactorl))
  (bind _returnvalue_2 (Actor|GetComponentbyClass _returnvalue "/Game/Blueprints/GrabComponent.GrabComponent_C"))
  (Utilities|IsValid _returnvalue :!pinned true ; Must be touching to attempt grab
    (:Is%20Valid
      (bind _isheld (Default|TryGrab _returnvalue_2 (Utilities|Select :Index HandType :NewEnumerator0 (Variables|Default|GetMotionControllerR) :NewEnumerator1 (Variables|Default|GetMotionControllerL))))
      (if _isheld ; Attempt grab
        (Utilities|FlowControl|Sequence
          (:then_0
            (switch Utilities|FlowControl|Switch|SwitchonHandType HandType ; Updage held component and reset if swapped from other
              (:NewEnumerator0
                (Variables|Default|SetHeldComponentR _returnvalue_2)
                (if (== (Variables|Default|GetHeldComponentL) (Variables|Default|GetHeldComponentR))
                  (Variables|Default|SetHeldComponentL 0)))
              (:NewEnumerator1
                (Variables|Default|SetHeldComponentL _returnvalue_2)
                (if (== (Variables|Default|GetHeldComponentL) (Variables|Default|GetHeldComponentR))
                  (Variables|Default|SetHeldComponentR 0)))))
          (:then_1
            (return true (Utilities|Select :Index HandType :NewEnumerator0 (Variables|Default|GetTouchedActorR) :NewEnumerator1 (Variables|Default|GetTouchedActorL))) ; Retrieve the correcponsing touched actor
          ))
        (else
          (return false 0))))
    (:Is%20Not%20Valid
      (return false 0))))

(fn CompleteGrabAction
  (params (HandType :type HandType%20Enum :default "NewEnumerator0"))
  (Utilities|IsValid (Utilities|Select :Index HandType :NewEnumerator0 (Variables|Default|GetHeldComponentR) :NewEnumerator1 (Variables|Default|GetHeldComponentL)) :!pinned true ; Must be holding a component to release
    (:Is%20Valid
      (bind _breleased (Default|TryRelease (Utilities|Select :Index HandType :NewEnumerator0 (Variables|Default|GetHeldComponentR) :NewEnumerator1 (Variables|Default|GetHeldComponentL))))
      (if _breleased
        (switch Utilities|FlowControl|Switch|SwitchonHandType HandType ; Reset the held components and\nretrieve the corresponding actor
          (:NewEnumerator0
            (Variables|Default|SetHeldComponentR 0)
            (return true (Variables|Default|GetTouchedActorR)))
          (:NewEnumerator1
            (Variables|Default|SetHeldComponentL 0)
            (return true (Variables|Default|GetTouchedActorL))))
        (else
          _)))
    (:Is%20Not%20Valid
      _))
  (return false 0))

(fn StartLinkAction
  (params (HandType :type HandType%20Enum :default "NewEnumerator0"))
  (bind _asbp_concept (Utilities|Casting|CastToBP_Concept (Utilities|Select :Index HandType :NewEnumerator0 (Variables|Default|GetTouchedActorR) :NewEnumerator1 (Variables|Default|GetTouchedActorL)) :!pinned true) ; Create link only if touching concept
    (:then
      (Utilities|FlowControl|Sequence
        (:then_0
          (bind _returnvalue (Game|SpawnActorfromClass "/Game/Blueprints/BP_Link.BP_Link_C" (Math|Transform|MakeTransform "0, 0, 0" "0, 0, 0" "1.000000,1.000000,1.000000") "Undefined" "MultiplyWithRoot" 0 0 :!pinned true)) ; Spawn link
          (bind _returnvalue_2 (Transformation|AttachActorToActor _returnvalue _asbp_concept "None" "KeepRelative" "KeepRelative" "KeepRelative" true :!pinned true)) ; Attach link to start point
        )
        (:then_1
          (bind _returnvalue_3 (Game|SpawnActorfromClass "/Game/Blueprints/BP_TempEndPoint.BP_TempEndPoint_C" (Math|Transform|MakeTransform "0, 0, 0" "0, 0, 0" "1.000000,1.000000,1.000000") "Undefined" "MultiplyWithRoot" 0 0 :!pinned true)) ; Spawn temporary end point
          (bind _returnvalue_4 (Transformation|AttachComponentToComponent _returnvalue_3 (Utilities|Select :Index HandType :NewEnumerator0 (Variables|Default|GetMotionControllerAimR) :NewEnumerator1 (Variables|Default|GetMotionControllerAimL)) "None" "KeepRelative" "KeepRelative" "KeepRelative" true :!pinned true)) ; Attach end point to controller
          (if (and _returnvalue_2 _returnvalue_4)
            (Default|SetEndActor _returnvalue _returnvalue_3 :!pinned true) ; Set end point as temporary point\nif seccessful
            (Default|SetVisibility _returnvalue true)
            (return true _returnvalue _asbp_concept)
            (else
              (Actor|DestroyActor _returnvalue_3 :!pinned true) ; Delete actors if failed to attach
              (Actor|DestroyActor _returnvalue)
              (return false 0 0))))))
    (:CastFailed
      (return false 0 0))))

(fn ConnectandValidateLink
  (params (Link :type BP%20Link%20Object%20Reference) (StartPoint :type Actor%20Object%20Reference) (HandType :type HandType%20Enum :default "NewEnumerator0"))
  (if (and (Utilities|IsValid Link) (Utilities|IsValid StartPoint)) ; Connect only if start\npoint and link exist
    (bind _asbp_concept (Utilities|Casting|CastToBP_Concept (Utilities|Select :Index HandType :NewEnumerator0 (Variables|Default|GetTouchedActorR) :NewEnumerator1 (Variables|Default|GetTouchedActorL))) ; End point must be a concept
      (:then
        (bind _asbp_concept_2 (Utilities|Casting|CastToBP_Concept StartPoint) ; start point must be a concept
          (:then
            (bind (_valid _link) (Default|CheckLink _asbp_concept_2 _asbp_concept :!pinned true)) ; Find if there exists a link between end points
            (if _valid
              ;[0 0 0] Destroy generated link
              (bind _endactor (Default|GetEndActor Link))
              (Actor|DestroyActor Link)
              (Actor|DestroyActor _endactor)
              (Default|SetVisibility _link true)
              (return true _asbp_concept true)
              (else
                ;[0 0 0] Set generated link end actor and schedule deletion
                (bind _endactor_2 (Default|GetEndActor Link))
                (Default|SetEndActor Link _asbp_concept)
                (Actor|DestroyActor _endactor_2)
                (Default|SetLinkColour Link "(R=1.000000,G=0.000000,B=0.029223,A=1.000000)")
                (Default|ActivateDeletion Link (Variables|Default|GetLinkTimeout))
                (return true _asbp_concept false))))
          (:CastFailed
            _)))
      (:CastFailed
        _))
    (else
      (Utilities|IsValid Link
        (:Is%20Valid
          _)
        (:Is%20Not%20Valid
          (return false 0 false)))))
  ;[0 0 0] Destroy generated link
  (bind _endactor_3 (Default|GetEndActor Link))
  (Actor|DestroyActor Link)
  (Actor|DestroyActor _endactor_3)
  (return false 0 false))

(fn ConfigureParameters
  (params (AllowLinkCreate :type Boolean))
  (Variables|Default|SetAllowLinkCreate AllowLinkCreate))